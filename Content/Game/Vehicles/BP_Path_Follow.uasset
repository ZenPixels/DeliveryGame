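; Vehicle component that drives its owning Chaos vehicle along a BP_Path spline, optionally auto-selecting the nearest at BeginPlay.
; Each tick projects an aim point ahead of the "routing" box onto the spline as the destination.
; Yaw error scaled by squared, clamped offset sets steering, which reduces throttle; StopZone applies the handbrake instead.
; Includes optional debug drawing and random next-spline selection, though its 90% progress trigger is unconnected.
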(event EventBeginPlay
  (Utilities|FlowControl|Sequence
    (:then_0
      (if (Variables|Default|GetAuto%20Find%20Spline)
        (bind _outactors (Actor|GetAllActorsOfClass "/Game/Game/Vehicles/BP_Path.BP_Path_C"))
        (bind _asbp_path (Utilities|Casting|CastToBP_Path (.ReturnValue (Actor|FindNearestActor (CallFunction|GetForwardAimLocation) _outactors))))
        (Variables|Default|SetTarget%20Spline _asbp_path)))
    (:then_1
      (bind _returnvalue (Game|AddComponentbyClass (Components|GetOwner) "/Script/Engine.TextRenderComponent" false (Math|Transform|MakeTransform (Math|Vector|MakeVector 0.0 0.0 (Math|Float|MakeLiteralFloat 275.0)) "0, 0, 0" "1.000000,1.000000,1.000000")))
      (bind _output_get (Variables|Default|SetText%20Render _returnvalue))
      (Rendering|Components|TextRender|SetTextRenderColor _output_get (Math|Color|MakeColor 1 1 1 1)))))

(event EventTick
  (params (DeltaSeconds :type Float%20%28single-precision%29))
  (CallFunction|GetCurrentDistanceonSpline)
  (CallFunction|UpdateDestination)
  (if (Variables|Default|GetStop%20Zone)
    (CallFunction|StopMoving)
    (else
      (CallFunction|ProceedtoDestination DeltaSeconds)))
  (if (Variables|Default|GetDraw%20Debug)
    (CallFunction|UpdateDebug)))

(fn GetForwardAimLocation
  (bind _returnvalue (Components|GetOwner))
  (return (+ (Transformation|GetWorldLocation (Utilities|Array|Get(acopy) (Actor|GetComponentsbyTag _returnvalue "/Script/Engine.BoxComponent" "routing"))) (* (Transformation|GetActorForwardVector _returnvalue) (Variables|Default|GetForward%20Aim%20Distance)))))

(fn GetCurrentDistanceonSpline
  (bind _target_spline (Variables|Default|GetTarget%20Spline))
  (bind _spline_path (Variables|/Game/Game/Vehicles/BP_Path.BP_Path_C|GetSpline%20Path _target_spline))
  (bind _output_get (Variables|Default|SetDistance%20Along%20Spline (Class|SplineComponent|GetDistanceAlongSplineatSplineInputKey _spline_path (Class|SplineComponent|FindInputKeyClosesttoWorldLocation _spline_path (Transformation|GetActorLocation (Components|GetOwner))))))
  (Variables|Default|SetPercentage%20Along%20Spline (* (/ _output_get (Spline|GetSplineLength _spline_path)) 1e+02)))

(fn UpdateDestination
  (Variables|Default|SetDestination (Spline|FindLocationClosesttoWorldLocation (Variables|/Game/Game/Vehicles/BP_Path.BP_Path_C|GetSpline%20Path (Variables|Default|GetTarget%20Spline)) (CallFunction|GetForwardAimLocation) "World")))

(fn UpdateDebug
  (Rendering|Debug|DrawDebugSphere (Variables|Default|GetDestination) 1e+01 12 "(R=1.000000,G=0.000000,B=0.000000,A=1.000000)" 0.0)
  (Rendering|Debug|DrawDebugSphere (CallFunction|GetForwardAimLocation) 1e+01 12 "(R=0.020612,G=0.152645,B=1.000000,A=1.000000)" 0.0)
  (Rendering|Components|TextRender|SetText (Variables|Default|GetText%20Render) (Utilities|Text|ToText(String) (Utilities|String|Append (Utilities|String|ToString(Integer) (Math|Float|Truncate (Variables|Default|GetDistance%20Along%20Spline))) " : " (Utilities|String|ToString(Integer) (Math|Float|Truncate (Variables|Default|GetPercentage%20Along%20Spline))) "% : " (Utilities|String|ToString(Float) (/ (Math|Conversions|ToFloat(Integer) (Math|Float|Floor (* (Variables|Default|GetSteering) 1e+02))) 1e+02)) " : " (Utilities|GetDisplayName (Variables|Default|GetTarget%20Spline)))))
  (Transformation|SetWorldRotation (Variables|Default|GetText%20Render) (Math|Conversions|RotationFromXVector (Math|Rotator|GetRotationXVector (* (Transformation|GetActorForwardVector (Game|GetPlayerController 0)) -1.0))) false false))

(fn ProceedtoDestination
  (params (Delta%20Time :type Float%20%28double-precision%29))
  (bind _returnvalue (Components|GetOwner))
  (bind _speed (Variables|Default|GetSpeed))
  (bind _returnvalue_2 (Actor|GetComponentbyClass _returnvalue "/Script/ChaosVehicles.ChaosVehicleMovementComponent"))
  (Variables|Default|SetTime%20Since%20Last%20Update Delta%20Time)
  (if (Utilities|IsValid _returnvalue_2)
    (Class|ChaosVehicleMovementComponent|SetHandbrakeInput _returnvalue_2 (or (not (Utilities|IsValid (Variables|Default|GetTarget%20Spline))) (Variables|Default|GetStop%20Zone)))
    (bind _output_get (Variables|Default|SetSteering (* (Math|Float|Power (Math|Float|Clamp(Float) (/ (Math|Vector|VectorLength (- (CallFunction|GetForwardAimLocation) (Variables|Default|GetDestination))) 1e+02)) 2.0) (Math|Float|MapRangeClamped (* (.yaw (Math|Rotator|Delta(Rotator) (Transformation|GetActorRotation (Components|GetOwner)) (Math|Rotator|FindLookatRotation (CallFunction|GetForwardAimLocation) (Variables|Default|GetDestination)))) 1.0) 1.2e+02 -1.2e+02 -1.0 1.0))))
    (Class|ChaosVehicleMovementComponent|SetSteeringInput _returnvalue_2 _output_get)
    (Class|ChaosVehicleMovementComponent|SetThrottleInput _returnvalue_2 (Math|Float|Clamp(Float) (* (- 1.1 (Math|Float|Absolute(Float) (Variables|Default|GetSteering))) _speed) 0.1 _speed))))

(fn GetNextTargetSpline
  (params (Target%20Splines :type Array%20of%20Object%20Object%20References))
  (Utilities|Array|RemoveItem Target%20Splines (Variables|Default|GetTarget%20Spline))
  (bind _asbp_path (Utilities|Casting|CastToBP_Path (.OutItem (Utilities|Array|Random Target%20Splines))))
  (Variables|Default|SetTarget%20Spline _asbp_path))

(fn StopMoving
  (Class|ChaosVehicleMovementComponent|SetHandbrakeInput (Actor|GetComponentbyClass (Components|GetOwner) "/Script/ChaosVehicles.ChaosVehicleMovementComponent") true))