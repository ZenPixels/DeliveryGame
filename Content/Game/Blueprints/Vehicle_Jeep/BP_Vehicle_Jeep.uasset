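; Drivable Chaos wheeled Jeep pawn that handles driving input, camera look and first/third-person toggle.
; Tick feeds engine RPM to a MetaSound and speed and RPM to the HUD, while hard hits trigger a crash sound.
; Possession toggles engine audio and the visible driver mesh.
; Exiting loops handbrake and negative throttle until stopped, blocking player throttle, then teleports the third-person character to the exit point and possesses it.
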(event OnComponentHit(Mesh)
  (params (HitComponent :type Primitive%20Component%20Object%20Reference) (OtherActor :type Actor%20Object%20Reference) (OtherComp :type Primitive%20Component%20Object%20Reference) (NormalImpulse :type Vector :default "0, 0, 0") (Hit :type Hit%20Result%20Structure%20%28by%20ref%29))
  (bind _returnvalue (Math|Vector|VectorLength NormalImpulse))
  (bind _returnvalue_2 (/ _returnvalue 1e+03))
  (Development|PrintString (Utilities|String|ToString(Float) _returnvalue_2))
  (if (> _returnvalue_2 1e+02)
    (Class|AudioParameterControllerInterface|SetTriggerParameter (Variables|Default|GetMetaSound_Car_Crash) "Reset Sound")
    (Audio|Components|Audio|Play (Variables|Default|GetMetaSound_Car_Crash) 0.0)
    (else
      (Class|AudioParameterControllerInterface|SetTriggerParameter (Variables|Default|GetMetaSound_Car_Crash) "Stop Sound"))))

(event Input|EnhancedActionEvents|EnhancedInputActionIA_Action
  (params (ActionValue :type Boolean) (ElapsedSeconds :type Float%20%28double-precision%29) (TriggeredSeconds :type Float%20%28double-precision%29) (InputAction :type Input%20Action%20Object%20Reference :default "/Game/Game/GameMode/IA_Action.IA_Action"))
  (bind _vehiclemovementcomponent (Variables|Default|GetVehicleMovementComponent))
  (bind _playerexit (Variables|Default|GetPlayerExit))
  (bind _returnvalue (Transformation|GetWorldTransform _playerexit))
  (:Started
    ;[1 1 1] Handbrake and reverse throttle until vehicle stops - note: vehicle pawn stops accepting input on unpossess
    (Variables|Default|SetIs%20Parking true) ; Restricts player input while stopping
    (Class|ChaosVehicleMovementComponent|SetHandbrakeInput _vehiclemovementcomponent true :!label _label)
    (Class|ChaosVehicleMovementComponent|SetThrottleInput _vehiclemovementcomponent -5e+02)
    (if (> (Math|Vector|VectorLength (Transformation|GetVelocity)) 0.0)
      (Utilities|FlowControl|Delay 0.1)
      (goto _label)
      (else
        ;[1 1 1] Place Player Actor on vehicle exit location
        (Variables|Default|SetIs%20Parking false) ; Resume player input
        (bind _returnvalue_2 (Actor|GetActorOfClass "/Game/Game/GameMode/BP_ThirdPersonCharacter_Main.BP_ThirdPersonCharacter_Main_C"))
        (Transformation|SetActorTransform _returnvalue_2 (Math|Transform|MakeTransform (.location _returnvalue) (.rotation _returnvalue) "1.000000,1.000000,1.000000") false true)
        (Pawn|Possess (Game|GetPlayerController 0) _returnvalue_2)))))

(event Input|EnhancedActionEvents|EnhancedInputActionIA_Toggle_Camera
  (params (ActionValue :type Boolean) (ElapsedSeconds :type Float%20%28double-precision%29) (TriggeredSeconds :type Float%20%28double-precision%29) (InputAction :type Input%20Action%20Object%20Reference :default "/Game/Game/GameMode/IA_Toggle_Camera.IA_Toggle_Camera"))
  (bind _first_person_camera (Variables|Default|GetFirst%20Person%20Camera))
  (bind _camera (Variables|Default|GetCamera))
  ;[1 1 1] Toggle Camera View
  (:Started
    (Utilities|FlowControl|FlipFlop
      (:A
        (Components|Activation|SetActive _first_person_camera true false)
        (Components|Activation|SetActive _camera false false))
      (:B
        (Components|Activation|SetActive _camera true false)
        (Components|Activation|SetActive _first_person_camera false false)))))

(event Input|EnhancedActionEvents|EnhancedInputActionIA_Handbrake
  (params (ActionValue :type Boolean) (ElapsedSeconds :type Float%20%28double-precision%29) (TriggeredSeconds :type Float%20%28double-precision%29) (InputAction :type Input%20Action%20Object%20Reference :default "/Game/Game/GameMode/IA_Handbrake.IA_Handbrake"))
  ;[1 1 1] Basic Verhicle Controls
  (:Triggered
    (Class|ChaosVehicleMovementComponent|SetHandbrakeInput (Variables|Default|GetVehicleMovementComponent) ActionValue :!label _label))
  (:Started
    (goto _label))
  (:Ongoing
    (goto _label))
  (:Completed
    (goto _label)))

(event Input|EnhancedActionEvents|EnhancedInputActionIA_Throttle
  (params (ActionValue :type Float%20%28double-precision%29) (ElapsedSeconds :type Float%20%28double-precision%29) (TriggeredSeconds :type Float%20%28double-precision%29) (InputAction :type Input%20Action%20Object%20Reference :default "/Game/Game/GameMode/IA_Throttle.IA_Throttle"))
  ;[1 1 1] Basic Verhicle Controls
  (:Triggered
    (if (== (Variables|Default|GetIs%20Parking) false) :!label _label
      (Class|ChaosVehicleMovementComponent|SetThrottleInput (Variables|Default|GetVehicleMovementComponent) ActionValue)))
  (:Completed
    (goto _label)))

(event Input|EnhancedActionEvents|EnhancedInputActionIA_Brake
  (params (ActionValue :type Float%20%28double-precision%29) (ElapsedSeconds :type Float%20%28double-precision%29) (TriggeredSeconds :type Float%20%28double-precision%29) (InputAction :type Input%20Action%20Object%20Reference :default "/Game/Game/GameMode/IA_Brake.IA_Brake"))
  ;[1 1 1] Basic Verhicle Controls
  (:Triggered
    (Class|ChaosVehicleMovementComponent|SetBrakeInput (Variables|Default|GetVehicleMovementComponent) ActionValue :!label _label))
  (:Completed
    (goto _label)))

(event Input|EnhancedActionEvents|EnhancedInputActionIA_Steering
  (params (ActionValue :type Float%20%28double-precision%29) (ElapsedSeconds :type Float%20%28double-precision%29) (TriggeredSeconds :type Float%20%28double-precision%29) (InputAction :type Input%20Action%20Object%20Reference :default "/Game/Game/GameMode/IA_Steering.IA_Steering"))
  ;[1 1 1] Basic Verhicle Controls
  (:Triggered
    (Class|ChaosVehicleMovementComponent|SetSteeringInput (Variables|Default|GetVehicleMovementComponent) ActionValue :!label _label))
  (:Started
    (goto _label))
  (:Canceled
    (goto _label))
  (:Completed
    (goto _label)))

(event EventTick
  (params (DeltaSeconds :type Float%20%28single-precision%29))
  ;[1 1 1] Feed RPM Rate into Engine Meta Sound Player
  (bind _aschaos_wheeled_vehicle_movement_component (Utilities|Casting|CastToChaosWheeledVehicleMovementComponent (Variables|Default|GetVehicleMovementComponent)))
  (Audio|Parameter|SetFloatParameter (Variables|Default|GetMetaSound_Engine) "RPM Range" (Math|Float|MapRangeClamped (Class|ChaosWheeledVehicleMovementComponent|GetEngineRotationSpeed _aschaos_wheeled_vehicle_movement_component) 1e+03 5e+03 0.0 1.0) :!class /Script/AudioExtensions.AudioParameterControllerInterface)
  (bind _asbp_hud_base (Utilities|Casting|CastToBP_HUD_Base (HUD|GetHUD (Game|GetPlayerController 0))))
  (bind (_mph _rpm) (CallFunction|GetVehicleStatus))
  (Default|UpdateDataValues (Variables|/Game/Game/UI/BP_HUD_Base.BP_HUD_Base_C|GetWB%20UI%20Vehicle _asbp_hud_base) _mph _rpm))

(event EventPossessed
  (params (NewController :type Controller%20Object%20Reference))
  (bind _driver (Variables|Default|GetDriver))
  ;[1 1 1] On Pawn Possessed start engine sound
  (Utilities|Casting|CastToPlayerController NewController)
  (Components|Activation|Activate (Variables|Default|GetMetaSound_Engine) true)
  (Variables|/Script/Engine.SkeletalMeshComponent|SetSkeletalMeshAsset _driver (Variables|Default|GetDriver%20Mesh))
  (Rendering|SetVisibility _driver true false))

(event EventUnpossessed
  (params (OldController :type Controller%20Object%20Reference))
  ;[1 1 1] On Pawn Unpossessed stop playing engine sound
  (Utilities|Casting|CastToPlayerController OldController)
  (Components|Activation|Deactivate (Variables|Default|GetMetaSound_Engine))
  (Rendering|SetVisibility (Variables|Default|GetDriver) false false))

(event Input|AxisEvents|InputAxisTurnRight/LeftMouse
  (params (AxisValue :type Float%20%28single-precision%29))
  ;[1 1 1] Camera Input - Mouse
  (Pawn|Input|AddControllerYawInput AxisValue))

(event Input|AxisEvents|InputAxisLookUp/DownMouse
  (params (AxisValue :type Float%20%28single-precision%29))
  ;[1 1 1] Camera Input - Mouse
  (Pawn|Input|AddControllerPitchInput AxisValue))

(event Input|GamepadEvents|GamepadRightX
  (params (AxisValue :type Float%20%28single-precision%29))
  ;[1 1 1] Camera Input - Mouse
  (Pawn|Input|AddControllerYawInput AxisValue))

(event Input|GamepadEvents|GamepadRightY
  (params (AxisValue :type Float%20%28single-precision%29))
  ;[1 1 1] Camera Input - Mouse
  (Pawn|Input|AddControllerPitchInput AxisValue))

(event Input|KeyboardEvents|1
  (params (Key :type Key%20Structure :default "None"))
  ;[1 1 1] Skin Change Test
  (:Pressed
    (Rendering|Components|Decal|SetDecalMaterial (Variables|Default|GetHood_Decal) "/Game/Game/Blueprints/Vehicle_Jeep/Decals/M_Veh_Decal_Unicorn.M_Veh_Decal_Unicorn")
    (Rendering|Material|SetMaterial (Variables|Character|GetMesh) 0 "/Game/Staging/AssetsvilleTown/Materials/MI_glossyOrange.MI_glossyOrange")))

(fn ConstructionScript)

(fn GetVehicleStatus
  (bind _aschaos_wheeled_vehicle_movement_component (Utilities|Casting|CastToChaosWheeledVehicleMovementComponent (Variables|Default|GetVehicleMovementComponent)))
  (return (Math|Float|Truncate (Class|ChaosVehicleMovementComponent|GetForwardSpeedMPH _aschaos_wheeled_vehicle_movement_component)) (Math|Float|Truncate (Class|ChaosWheeledVehicleMovementComponent|GetEngineRotationSpeed _aschaos_wheeled_vehicle_movement_component))))