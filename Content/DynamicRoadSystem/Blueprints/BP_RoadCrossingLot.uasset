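; Editor-generated road crossing lot for the dynamic road system, built as a dynamic mesh from a closed spline outline.
; On rebuild it snaps spline points to the ground with line traces, then sweeps edge profiles and fills holes using Geometry Script.
; First-time OSM imports get their winding checked and reversed if needed.
; It can bake to a static mesh asset with optional Nanite, and rebuilds attached road connectors.
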(event Custom|Force%20Rebuild
  (bind _returnvalue (Math|DateTime|Now))
  (bind _returnvalue_2 (Transformation|GetActorRotation))
  (bind _spline (Variables|Default|GetSpline))
  (bind _spline_2 (Variables|Default|GetSpline))
  (bind _curve_scaler (Variables|DynamicMeshOptions|GetCurve%20Scaler))
  (bind _returnvalue_3 (Spline|GetNumberOfSplinePoints _spline_2))
  (bind _returnvalue_4 (- _returnvalue_3 1))
  (bind _returnvalue_5 (DynamicMeshComponent|GetDynamicMesh (Variables|DynamicMeshActor|GetDynamicMeshComponent)))
  (Variables|DynamicMeshOptions|SetTarget%20Mesh _returnvalue_5)
  (if (Variables|DynamicMeshOptions|GetShow%20Function%20Completion%20Time)
    (Variables|Default|SetDebugTime (Math|DateTime|Now)))
  ;[1 1 1] Sets the amounts of desired triangles when making the dynamic mesh based off how long the mesh is
  (Variables|Default|SetAutoResolution (Math|Float|Truncate (* (+ (/ (Spline|GetSplineLength (Variables|Default|GetSpline)) 1e+01) 1e+01) (Variables|DynamicMeshOptions|GetResolution%20Multiplier))))
  ;[1 1 1] Do not allow xy rotation when snapping is enabled. It just moves the points closer to the pivot origin point due to the ground snapping
  (if (and (not (Variables|DynamicMeshOptions|GetDisable%20Ground%20Snapping)) (or (!= (.roll _returnvalue_2) 0.0) (!= (.pitch _returnvalue_2) 0.0)))
    (Transformation|SetActorRotation (Math|Rotator|MakeRotator 0.0 0.0 (.yaw _returnvalue_2))))
  (bind _return (CallFunction|DisplayStaticMesh?))
  (if (not _return)
    ;[1 1 1] Corrects array direction if OSM points inverts geometry
    (if (Variables|OSM|GetFlipGeometry)
      (Utilities|Array|Reverse (Variables|DynamicMeshOptions|GetRoad%20Points%20Override))
      (Variables|OSM|SetFlipGeometry false))
    ;[1 1 1] If the user overrides a road point then update the spline point
    (if (Utilities|Array|Identical (Variables|DynamicMeshOptions|GetRoad%20Points%20Override) (Variables|DynamicMeshOptions|GetRoadPoints))
      _
      (else
        (Spline|SetSplinePoints (Variables|Default|GetSpline) (Variables|DynamicMeshOptions|GetRoad%20Points%20Override) "World" true)
        (Variables|DynamicMeshOptions|SetRoadPoints (Variables|DynamicMeshOptions|GetRoad%20Points%20Override))))
    ;[1 1 1] Check if user added or deleted spline point and add it to an array
    (if (== _returnvalue_3 (Utilities|Array|Length (Variables|DynamicMeshOptions|GetRoadPoints)))
      _
      (else
        (Utilities|Array|Clear (Variables|DynamicMeshOptions|GetRoadPoints))
        (for _index (range 0 _returnvalue_4)
          (Utilities|Array|SetArrayElem (Variables|DynamicMeshOptions|GetRoadPoints) _index (Spline|GetLocationatSplinePoint (Variables|Default|GetSpline) _returnvalue_4 "World") true))))
    ;[1 1 1] Save Road Point Positions
    (for _index_2 (range 0 (- (Spline|GetNumberOfSplinePoints _spline) 1))
      (Utilities|Array|SetArrayElem (Variables|DynamicMeshOptions|GetRoadPoints) _index_2 (Math|Vector|MakeVector (.x (Spline|GetLocationatSplinePoint _spline _index_2 "World")) (.y (Spline|GetLocationatSplinePoint _spline _index_2 "World")) (.z (Utilities|Array|Get(acopy) (Variables|DynamicMeshOptions|GetRoadPoints) _index_2))) true))
    (if (Variables|DynamicMeshOptions|GetDisable%20Ground%20Snapping)
      _
      (else
        (Spline|SetSplinePoints (Variables|Default|GetSpline) (Variables|DynamicMeshOptions|GetRoadPoints) "World" true)))
    ;[1 1 1] Locks spline points to the landscape
    (for (_ _array_index) (Variables|DynamicMeshOptions|GetRoadPoints)
      (CallFunction|SnapRoadtoGround _array_index))
    (Spline|SetSplinePoints (Variables|Default|GetSpline) (Variables|DynamicMeshOptions|GetRoadPoints) "World" true)
    ;[1 1 1] Set Tangents equal to zero in parts of road that are not supposed to curve as much
    (if (!= (Variables|DynamicMeshOptions|GetCurve%20Scaler) 1.0)
      (for _index_3 (range 0 (- (Spline|GetNumberOfSplinePoints (Variables|Default|GetSpline)) 1))
        (Spline|SetTangentatSplinePoint (Variables|Default|GetSpline) _index_3 (/ (Spline|GetTangentatSplinePoint (Variables|Default|GetSpline) _index_3 "World") (Math|Vector|MakeVector _curve_scaler _curve_scaler _curve_scaler)) "World" true)))
    (if (and (Utilities|Map|IsNotEmpty (Variables|OSM|GetOSMTags)) (Variables|OSM|GetFirstTimeImport))
      (CallFunction|GeometryCorrection))
    (bind _target_mesh (CallFunction|MakeDynamicMesh))
    (CallFunction|BaketoStaticMesh _target_mesh)
    (CallFunction|UpdateConnectedRoadstoSelf)
    (Variables|OSM|SetFirstTimeImport false)
    (if (Variables|DynamicMeshOptions|GetReset%20Pivot%20Point)
      (CallFunction|ResetPivot))
    (Variables|DynamicMeshOptions|SetRoad%20Points%20Override (Variables|DynamicMeshOptions|GetRoadPoints))
    ;[1 1 1] debug amount of time for function
    (if (Variables|DynamicMeshOptions|GetShow%20Function%20Completion%20Time)
      (Development|PrintString (Utilities|String|Append "Function took x milliseconds: " (Utilities|String|ToString(Integer) (+ (- (* (.minute _returnvalue) 60000) (* (.minute (Variables|Default|GetDebugTime)) 60000)) (- (* (.second _returnvalue) 1000) (* (.second (Variables|Default|GetDebugTime)) 1000)) (- (.millisecond _returnvalue) (.millisecond (Variables|Default|GetDebugTime)))))) false))))

(event Events|EventOnRebuildGeneratedMesh
  (params (TargetMesh :type Dynamic%20Mesh%20Object%20Reference))
  (bind _returnvalue (Math|DateTime|Now))
  (bind _returnvalue_2 (Transformation|GetActorRotation))
  (bind _spline (Variables|Default|GetSpline))
  (bind _spline_2 (Variables|Default|GetSpline))
  (bind _curve_scaler (Variables|DynamicMeshOptions|GetCurve%20Scaler))
  (bind _returnvalue_3 (Spline|GetNumberOfSplinePoints _spline_2))
  (bind _returnvalue_4 (- _returnvalue_3 1))
  (Variables|DynamicMeshOptions|SetTarget%20Mesh TargetMesh)
  (if (Variables|DynamicMeshOptions|GetShow%20Function%20Completion%20Time)
    (Variables|Default|SetDebugTime (Math|DateTime|Now)))
  ;[1 1 1] Sets the amounts of desired triangles when making the dynamic mesh based off how long the mesh is
  (Variables|Default|SetAutoResolution (Math|Float|Truncate (* (+ (/ (Spline|GetSplineLength (Variables|Default|GetSpline)) 1e+01) 1e+01) (Variables|DynamicMeshOptions|GetResolution%20Multiplier))))
  ;[1 1 1] Do not allow xy rotation when snapping is enabled. It just moves the points closer to the pivot origin point due to the ground snapping
  (if (and (not (Variables|DynamicMeshOptions|GetDisable%20Ground%20Snapping)) (or (!= (.roll _returnvalue_2) 0.0) (!= (.pitch _returnvalue_2) 0.0)))
    (Transformation|SetActorRotation (Math|Rotator|MakeRotator 0.0 0.0 (.yaw _returnvalue_2))))
  (bind _return (CallFunction|DisplayStaticMesh?))
  (if (not _return)
    ;[1 1 1] Corrects array direction if OSM points inverts geometry
    (if (Variables|OSM|GetFlipGeometry)
      (Utilities|Array|Reverse (Variables|DynamicMeshOptions|GetRoad%20Points%20Override))
      (Variables|OSM|SetFlipGeometry false))
    ;[1 1 1] If the user overrides a road point then update the spline point
    (if (Utilities|Array|Identical (Variables|DynamicMeshOptions|GetRoad%20Points%20Override) (Variables|DynamicMeshOptions|GetRoadPoints))
      _
      (else
        (Spline|SetSplinePoints (Variables|Default|GetSpline) (Variables|DynamicMeshOptions|GetRoad%20Points%20Override) "World" true)
        (Variables|DynamicMeshOptions|SetRoadPoints (Variables|DynamicMeshOptions|GetRoad%20Points%20Override))))
    ;[1 1 1] Check if user added or deleted spline point and add it to an array
    (if (== _returnvalue_3 (Utilities|Array|Length (Variables|DynamicMeshOptions|GetRoadPoints)))
      _
      (else
        (Utilities|Array|Clear (Variables|DynamicMeshOptions|GetRoadPoints))
        (for _index (range 0 _returnvalue_4)
          (Utilities|Array|SetArrayElem (Variables|DynamicMeshOptions|GetRoadPoints) _index (Spline|GetLocationatSplinePoint (Variables|Default|GetSpline) _returnvalue_4 "World") true))))
    ;[1 1 1] Save Road Point Positions
    (for _index_2 (range 0 (- (Spline|GetNumberOfSplinePoints _spline) 1))
      (Utilities|Array|SetArrayElem (Variables|DynamicMeshOptions|GetRoadPoints) _index_2 (Math|Vector|MakeVector (.x (Spline|GetLocationatSplinePoint _spline _index_2 "World")) (.y (Spline|GetLocationatSplinePoint _spline _index_2 "World")) (.z (Utilities|Array|Get(acopy) (Variables|DynamicMeshOptions|GetRoadPoints) _index_2))) true))
    (if (Variables|DynamicMeshOptions|GetDisable%20Ground%20Snapping)
      _
      (else
        (Spline|SetSplinePoints (Variables|Default|GetSpline) (Variables|DynamicMeshOptions|GetRoadPoints) "World" true)))
    ;[1 1 1] Locks spline points to the landscape
    (for (_ _array_index) (Variables|DynamicMeshOptions|GetRoadPoints)
      (CallFunction|SnapRoadtoGround _array_index))
    (Spline|SetSplinePoints (Variables|Default|GetSpline) (Variables|DynamicMeshOptions|GetRoadPoints) "World" true)
    ;[1 1 1] Set Tangents equal to zero in parts of road that are not supposed to curve as much
    (if (!= (Variables|DynamicMeshOptions|GetCurve%20Scaler) 1.0)
      (for _index_3 (range 0 (- (Spline|GetNumberOfSplinePoints (Variables|Default|GetSpline)) 1))
        (Spline|SetTangentatSplinePoint (Variables|Default|GetSpline) _index_3 (/ (Spline|GetTangentatSplinePoint (Variables|Default|GetSpline) _index_3 "World") (Math|Vector|MakeVector _curve_scaler _curve_scaler _curve_scaler)) "World" true)))
    (if (and (Utilities|Map|IsNotEmpty (Variables|OSM|GetOSMTags)) (Variables|OSM|GetFirstTimeImport))
      (CallFunction|GeometryCorrection))
    (bind _target_mesh (CallFunction|MakeDynamicMesh))
    (CallFunction|BaketoStaticMesh _target_mesh)
    (CallFunction|UpdateConnectedRoadstoSelf)
    (Variables|OSM|SetFirstTimeImport false)
    (if (Variables|DynamicMeshOptions|GetReset%20Pivot%20Point)
      (CallFunction|ResetPivot))
    (Variables|DynamicMeshOptions|SetRoad%20Points%20Override (Variables|DynamicMeshOptions|GetRoadPoints))
    ;[1 1 1] debug amount of time for function
    (if (Variables|DynamicMeshOptions|GetShow%20Function%20Completion%20Time)
      (Development|PrintString (Utilities|String|Append "Function took x milliseconds: " (Utilities|String|ToString(Integer) (+ (- (* (.minute _returnvalue) 60000) (* (.minute (Variables|Default|GetDebugTime)) 60000)) (- (* (.second _returnvalue) 1000) (* (.second (Variables|Default|GetDebugTime)) 1000)) (- (.millisecond _returnvalue) (.millisecond (Variables|Default|GetDebugTime)))))) false))))

(fn ConstructionScript)

(fn BaketoStaticMesh
  (params (FromDynamicMesh :type Dynamic%20Mesh%20Object%20Reference))
  (bind _meshnanitesettings (Utilities|Struct|MakeMeshNaniteSettings true))
  (bind _dynamicmeshcomponent (Variables|DynamicMeshActor|GetDynamicMeshComponent))
  (bind _staticmesh (Variables|Default|GetStaticMesh))
  (bind _returnvalue (Rendering|Material|GetMaterials _dynamicmeshcomponent))
  ;[1 1 1] Bake to static mesh
  (if (Variables|StaticMeshOptions|GetBakeToStaticMesh)
    (Variables|StaticMeshOptions|SetBakeToStaticMesh false)
    (bind _returnvalue_2 (Game|GetCurrentLevelName true))
    (bind _output_get (Variables|StaticMeshOptions|SetStatic%20Mesh%20Asset%20Path (Utilities|String|Append "/Game/RoadStaticMeshes/" _returnvalue_2 "/" (Utilities|GetDisplayName self))))
    (bind _returnvalue_3 (EditorScripting|Asset|DoesAssetExist _output_get :!class /Script/EditorScriptingUtilities.EditorAssetLibrary))
    (if (not _returnvalue_3)
      (bind _returnvalue_4 (GeometryScript|AssetManagement|CreateNewStaticMeshAssetfromMesh FromDynamicMesh _output_get (Utilities|Struct|MakeGeometryScriptCreateNewStaticMeshAssetOptions false false (Variables|StaticMeshOptions|GetEnable%20Nanite) _meshnanitesettings 0.0 true "CTF_UseComplexAsSimple") 0) ; Create new asset since it does not exist
        (:Failure
          _)
        (:Success
          (Variables|StaticMeshOptions|SetTo%20Static%20Mesh%20Asset _returnvalue_4)
          (Components|StaticMesh|SetStaticMesh _staticmesh _returnvalue_4)
          (Rendering|SetVisibility _staticmesh false false)
          (Development|PrintString "Success" false :!label _label)
          (if (Variables|StaticMeshOptions|GetCopy%20Materials)
            (for _index (range 0 (- (Utilities|Array|Length _returnvalue) 1))
              (Rendering|Material|SetMaterial (Variables|StaticMeshOptions|GetTo%20Static%20Mesh%20Asset) _index (Utilities|Array|Get(acopy) _returnvalue _index)))
            (return)
            (else
              (return)))))
      (else
        (GeometryScript|StaticMesh|CopyMeshtoStaticMesh :FromDynamicMesh FromDynamicMesh :ToStaticMeshAsset (Variables|StaticMeshOptions|GetTo%20Static%20Mesh%20Asset) :Options (Utilities|Struct|MakeGeometryScriptCopyMeshtoAssetOptions false false false false 0 0 (Variables|StaticMeshOptions|GetEnable%20Nanite) "(bEnabled=True,FallbackPercentTriangles=100.000000,FallbackRelativeError=0.000000)" _meshnanitesettings true false) :Debug 0 ; Use existing asset and update it
          (:Failure
            _)
          (:Success
            (goto _label)))))
    (Development|PrintString "Failure to convert to static mesh")
    (return)
    (else
      (return))))

(fn SnapRoadtoGround
  (params (index :type Integer))
  (bind _returnvalue (Transformation|GetActorLocation))
  (bind _trace_distance (Variables|DynamicMeshOptions|GetTrace%20Distance))
  (bind _spline (Variables|Default|GetSpline))
  (bind _roadpoints (Variables|DynamicMeshOptions|GetRoadPoints))
  (bind _roadpoints_2 (Variables|DynamicMeshOptions|GetRoadPoints))
  (bind _returnvalue_2 (Spline|GetLocationatSplinePoint _spline index "World"))
  (bind _output (Utilities|Array|Get(acopy) _roadpoints_2 index))
  (bind _output_2 (Utilities|Array|Get(acopy) _roadpoints index))
  (bind _returnvalue_3 (Math|Vector|MakeVector (.x _returnvalue_2) (.y _returnvalue_2) (.z _returnvalue)))
  (if (Variables|DynamicMeshOptions|GetDisable%20Ground%20Snapping)
    (Utilities|Array|SetArrayElem _roadpoints_2 index (Math|Vector|MakeVector (.x _output) (.y _output) (.z (Spline|GetLocationatSplinePoint (Variables|Default|GetSpline) index "World"))))
    (return)
    (else
      (bind (_outhit _returnvalue_4) (Collision|LineTraceByChannel (+ (Math|Vector|MakeVector 0.0 0.0 _trace_distance) _returnvalue_3) (+ (Math|Vector|MakeVector 0.0 0.0 (* _trace_distance -1.0)) _returnvalue_3) "TraceTypeQuery1" true (Variables|DynamicMeshOptions|GetActors%20to%20Ignore%20when%20Tracing) "None"))
      (if _returnvalue_4
        (Utilities|Array|SetArrayElem _roadpoints index (Math|Vector|MakeVector (.x _output_2) (.y _output_2) (.z (.impactpoint _outhit))))
        (return)
        (else
          (return))))))

(fn DisplayStaticMesh?
  ;[1 1 1] Determines whether static mesh is being previewed and sets relevant data
  (if (Variables|StaticMeshOptions|GetPreview%20Static%20Mesh)
    (Rendering|SetVisibility (Variables|Default|GetStaticMesh) true false)
    (Development|PrintString "Static Mesh Active any other variable changes will not be reflected" false)
    (return true)
    (else
      (if (Rendering|IsVisible (Variables|Default|GetStaticMesh))
        (Rendering|SetVisibility (Variables|Default|GetStaticMesh) false false))
      (return false))))

(fn MakeDynamicMesh
  (bind _road_height_scale (Variables|DynamicMeshOptions|GetRoad%20Height%20Scale))
  (bind _returnvalue (* _road_height_scale 25.0))
  (DynamicMesh|Reset (Variables|DynamicMeshOptions|GetTarget%20Mesh))
  (bind _frames (Class|GeometryScriptLibraryPolyPathFunctions|SampleSplinetoTransforms :Spline (Variables|Default|GetSpline) :SamplingOptions (Utilities|Struct|MakeGeometryScriptSplineSamplingOptions (Variables|Default|GetAutoResolution) 1.0 "UniformDistance" "World")))
  (bind _returnvalue_2 (DynamicMeshActor|AllocateComputeMesh))
  (bind _returnvalue_3 (GeometryScript|Primitives|AppendSweepPolyline :TargetMesh _returnvalue_2 :Transform (Math|Transform|MakeTransform (* (Transformation|GetActorLocation) "-1.000000,-1.000000,-1.000000") "0, 0, 0" "1.000000,1.000000,1.000000") :PolylineVertices (Utilities|Array|MakeArray (Math|Vector2D|MakeVector2D 2e+01 0.0) (Math|Vector2D|MakeVector2D 0.0 (* (Variables|DynamicMeshOptions|GetRoad%20Height%20Scale) 25.0))) :SweepPath _frames :bLoop true :Debug 0))
  (GeometryScript|MeshEdits|AppendMesh :TargetMesh (Variables|DynamicMeshOptions|GetTarget%20Mesh) :AppendMesh _returnvalue_3 :AppendOptions "(CombineMode=EnableAllMatching)" :Debug 0)
  (DynamicMeshActor|ReleaseAllComputeMeshes)
  (bind _returnvalue_4 (Class|GeometryScriptLibraryMeshRepairFunctions|FillAllMeshHoles (Variables|DynamicMeshOptions|GetTarget%20Mesh) (Utilities|Struct|MakeGeometryScriptFillHolesOptions "PlanarProjection") 0))
  (bind _returnvalue_5 (Class|GeometryScriptLibraryMeshPrimitiveFunctions|AppendSweepPolygon :TargetMesh _returnvalue_4 :Transform (Math|Transform|MakeTransform (* (Transformation|GetActorLocation) "-1.000000,-1.000000,-1.000000") "0, 0, 0" "1.000000,1.000000,1.000000") :PolygonVertices (Utilities|Array|MakeArray (Math|Vector2D|MakeVector2D 2e+01 0.0) (Math|Vector2D|MakeVector2D 1e+01 (* _returnvalue 0.8)) (Math|Vector2D|MakeVector2D 0.0 _returnvalue)) :SweepPath _frames :bLoop true :bCapped false :Debug 0))
  (bind _returnvalue_6 (Class|GeometryScriptLibraryMeshRepairFunctions|FillAllMeshHoles _returnvalue_5 (Utilities|Struct|MakeGeometryScriptFillHolesOptions "PlanarProjection") 0))
  (Class|GeometryScriptLibraryMeshTransformFunctions|RotateMesh _returnvalue_6 (* (Transformation|GetActorRotation) -1.0) "0.000000,0.000000,0.000000" 0)
  (return _returnvalue_6))

(fn UpdateConnectedRoadstoSelf
  (bind _road_connector (Variables|DynamicMeshOptions|GetRoad%20Connector))
  ;[1 1 1] Update all BP_RoadConnection blueprints attached to this actor if "Update Connected Roads" is true
  (if (Variables|DynamicMeshOptions|GetUpdate%20Connected%20Roads)
    (for _array_element _road_connector
      (if (Utilities|IsValid _array_element)
        (if (== (.connectedcrossinglot (Variables|/Game/DynamicRoadSystem/Blueprints/BP_RoadConnection.BP_RoadConnection_C|GetMainConnectedRoad _array_element)) self)
          (Default|ForceRebuild _array_element)
          (else
            (Utilities|Array|RemoveItem _road_connector _array_element :!label _label)))
        (else
          (goto _label))))
    (return)
    (else
      (return))))

(fn GeometryCorrection
  (bind _roadpoints (Variables|DynamicMeshOptions|GetRoadPoints))
  (bind _roadpoints_2 (Variables|DynamicMeshOptions|GetRoadPoints))
  (bind _curve_scaler (Variables|DynamicMeshOptions|GetCurve%20Scaler))
  (LocalVariables|SetFurthestWestPoint 9999999999.0)
  (for (_array_element _array_index) _roadpoints_2
    (if (< (.y _array_element) (LocalVariables|GetFurthestWestPoint))
      (LocalVariables|SetFWPIndex _array_index :!label _label)
      (LocalVariables|SetFurthestWestPoint (.y _array_element))
      (elif (== (LocalVariables|GetFurthestWestPoint) (.y _array_element)) ; if two indexes share the same y coord use the point with the lower x
        (if (< (.x _array_element) (.x (Utilities|Array|Get(acopy) (Variables|DynamicMeshOptions|GetRoadPoints) (LocalVariables|GetFWPIndex))))
          (goto _label)))))
  (if (== (LocalVariables|GetFWPIndex) 0)
    (LocalVariables|SetFWPUpperIndex (+ (LocalVariables|GetFWPIndex) 1))
    (LocalVariables|SetFWPLowerIndex (- (Utilities|Array|Length (Variables|DynamicMeshOptions|GetRoadPoints)) 1))
    (elif (== (LocalVariables|GetFWPIndex) (- (Utilities|Array|Length _roadpoints_2) 1))
      (LocalVariables|SetFWPUpperIndex 0)
      (LocalVariables|SetFWPLowerIndex (- (LocalVariables|GetFWPIndex) 1))
      (else
        (LocalVariables|SetFWPUpperIndex (+ (LocalVariables|GetFWPIndex) 1))
        (LocalVariables|SetFWPLowerIndex (- (LocalVariables|GetFWPIndex) 1)))))
  (if (== (- (.y (Utilities|Array|Get(acopy) _roadpoints (LocalVariables|GetFWPUpperIndex))) (.y (Utilities|Array|Get(acopy) _roadpoints (LocalVariables|GetFWPIndex)))) 0.0)
    _
    (elif (== (- (.y (Utilities|Array|Get(acopy) _roadpoints (LocalVariables|GetFWPLowerIndex))) (.y (Utilities|Array|Get(acopy) _roadpoints (LocalVariables|GetFWPIndex)))) 0.0)
      (return)
      (elif (> (/ (- (.x (Utilities|Array|Get(acopy) _roadpoints (LocalVariables|GetFWPUpperIndex))) (.x (Utilities|Array|Get(acopy) _roadpoints (LocalVariables|GetFWPIndex)))) (- (.y (Utilities|Array|Get(acopy) _roadpoints (LocalVariables|GetFWPUpperIndex))) (.y (Utilities|Array|Get(acopy) _roadpoints (LocalVariables|GetFWPIndex))))) (/ (- (.x (Utilities|Array|Get(acopy) _roadpoints (LocalVariables|GetFWPLowerIndex))) (.x (Utilities|Array|Get(acopy) _roadpoints (LocalVariables|GetFWPIndex)))) (- (.y (Utilities|Array|Get(acopy) _roadpoints (LocalVariables|GetFWPLowerIndex))) (.y (Utilities|Array|Get(acopy) _roadpoints (LocalVariables|GetFWPIndex))))))
        _
        (else
          (return)))))
  ;[1 1 1] Invert Geometry
  (Utilities|Array|Reverse (Variables|DynamicMeshOptions|GetRoad%20Points%20Override))
  (Utilities|Array|Reverse (Variables|DynamicMeshOptions|GetRoadPoints))
  (Spline|SetSplinePoints (Variables|Default|GetSpline) (Variables|DynamicMeshOptions|GetRoadPoints) "World" true)
  ;[1 1 1] Set Tangents equal to zero in parts of road that are not supposed to curve as much
  (if (!= (Variables|DynamicMeshOptions|GetCurve%20Scaler) 1.0)
    (for _index (range 0 (- (Spline|GetNumberOfSplinePoints (Variables|Default|GetSpline)) 1))
      (Spline|SetTangentatSplinePoint (Variables|Default|GetSpline) _index (/ (Spline|GetTangentatSplinePoint (Variables|Default|GetSpline) _index "World") (Math|Vector|MakeVector _curve_scaler _curve_scaler _curve_scaler)) "World" true)))
  (return))

(fn ResetPivot
  (bind _spline (Variables|Default|GetSpline))
  (bind _returnvalue (Spline|GetLocationatSplinePoint _spline 0 "World"))
  (LocalVariables|SetOffset (- (Transformation|GetActorLocation) _returnvalue))
  (Transformation|SetActorLocation _returnvalue false false)
  (Transformation|AddWorldOffset (Variables|Default|GetSpline) (LocalVariables|GetOffset) false false)
  (Variables|DynamicMeshOptions|SetReset%20Pivot%20Point false)
  (Spline|SetSplinePoints (Variables|Default|GetSpline) (Variables|DynamicMeshOptions|GetRoadPoints) "World" true)
  (CallFunction|ForceRebuild))