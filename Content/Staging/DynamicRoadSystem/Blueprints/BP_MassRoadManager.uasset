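; Manager actor for batch operations on every road system, connection and crossing lot in the level of the dynamic road system.
; It force-rebuilds roads with optional resolution override, bakes them to static meshes with optional Nanite, or spawns StaticMeshActors from baked assets, optionally deleting the originals.
; It also reports overlaps via vertical line traces along road points and extends lane lines at connections for OSM roads.
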(fn ConstructionScript)

(fn PrintRoadCount
  (Utilities|FlowControl|Sequence
    (:then_0
      (bind _outactors (Actor|GetAllActorsOfClass "/Game/Staging/DynamicRoadSystem/Blueprints/BP_RoadSystem.BP_RoadSystem_C"))
      (Development|PrintString (Utilities|String|Append "There are " (Utilities|String|ToString(Integer) (Utilities|Array|Length _outactors)) " main road systems")))
    (:then_1
      (bind _outactors_2 (Actor|GetAllActorsOfClass "/Game/Staging/DynamicRoadSystem/Blueprints/BP_RoadConnection.BP_RoadConnection_C"))
      (Development|PrintString (Utilities|String|Append "There are " (Utilities|String|ToString(Integer) (Utilities|Array|Length _outactors_2)) " main road connections")))
    (:then_2
      (bind _outactors_3 (Actor|GetAllActorsOfClass "/Game/Staging/DynamicRoadSystem/Blueprints/BP_RoadCrossingLot.BP_RoadCrossingLot_C"))
      (Development|PrintString (Utilities|String|Append "There are " (Utilities|String|ToString(Integer) (Utilities|Array|Length _outactors_3)) " main road lots")))))

(fn ReplaceAllDynamicwithStatic
  (Utilities|FlowControl|Sequence
    (:then_0
      (bind _outactors (Actor|GetAllActorsOfClass "/Game/Staging/DynamicRoadSystem/Blueprints/BP_RoadSystem.BP_RoadSystem_C"))
      (for _array_element _outactors
        (bind _to_static_mesh_asset (Variables|/Game/Staging/DynamicRoadSystem/Blueprints/BP_RoadSystem.BP_RoadSystem_C|GetTo%20Static%20Mesh%20Asset _array_element)
          (:then
            (bind _returnvalue (Game|SpawnActorfromClass "/Script/Engine.StaticMeshActor" (Transformation|GetActorTransform _array_element) "AlwaysSpawn" "MultiplyWithRoot" 0 0))
            (Components|StaticMesh|SetStaticMesh (Variables|/Script/Engine.StaticMeshActor|GetStaticMeshComponent _returnvalue) _to_static_mesh_asset)
            (if (Variables|Replacing|GetDelete%20Dynamic%20when%20Done)
              (Actor|DestroyActor _array_element)))
          (:else))))
    (:then_1
      (bind _outactors_2 (Actor|GetAllActorsOfClass "/Game/Staging/DynamicRoadSystem/Blueprints/BP_RoadConnection.BP_RoadConnection_C"))
      (for _array_element_2 _outactors_2
        (bind _to_static_mesh_asset_2 (Variables|/Game/Staging/DynamicRoadSystem/Blueprints/BP_RoadConnection.BP_RoadConnection_C|GetTo%20Static%20Mesh%20Asset _array_element_2)
          (:then
            (bind _returnvalue_2 (Game|SpawnActorfromClass "/Script/Engine.StaticMeshActor" (Transformation|GetActorTransform _array_element_2) "AlwaysSpawn" "MultiplyWithRoot" 0 0))
            (Components|StaticMesh|SetStaticMesh (Variables|/Script/Engine.StaticMeshActor|GetStaticMeshComponent _returnvalue_2) _to_static_mesh_asset_2)
            (if (Variables|Replacing|GetDelete%20Dynamic%20when%20Done)
              (Actor|DestroyActor _array_element_2)))
          (:else))))
    (:then_2
      (bind _outactors_3 (Actor|GetAllActorsOfClass "/Game/Staging/DynamicRoadSystem/Blueprints/BP_RoadCrossingLot.BP_RoadCrossingLot_C"))
      (for _array_element_3 _outactors_3
        (bind _to_static_mesh_asset_3 (Variables|/Game/Staging/DynamicRoadSystem/Blueprints/BP_RoadCrossingLot.BP_RoadCrossingLot_C|GetTo%20Static%20Mesh%20Asset _array_element_3)
          (:then
            (bind _returnvalue_3 (Game|SpawnActorfromClass "/Script/Engine.StaticMeshActor" (Transformation|GetActorTransform _array_element_3) "AlwaysSpawn" "MultiplyWithRoot" 0 0))
            (Components|StaticMesh|SetStaticMesh (Variables|/Script/Engine.StaticMeshActor|GetStaticMeshComponent _returnvalue_3) _to_static_mesh_asset_3)
            (if (Variables|Replacing|GetDelete%20Dynamic%20when%20Done)
              (Actor|DestroyActor _array_element_3)))
          (:else))))))

(fn BakeAllRoadstoStaticMesh
  (bind _returnvalue (Math|DateTime|Now))
  ;[1 1 1] Debug time
  (LocalVariables|SetDebug%20Time (Math|DateTime|Now))
  (Utilities|FlowControl|Sequence
    (:then_0
      (bind _outactors (Actor|GetAllActorsOfClass "/Game/Staging/DynamicRoadSystem/Blueprints/BP_RoadSystem.BP_RoadSystem_C"))
      (for _array_element _outactors
        (Variables|/Game/Staging/DynamicRoadSystem/Blueprints/BP_RoadSystem.BP_RoadSystem_C|SetResolution%20Multiplier _array_element (* (Variables|/Game/Staging/DynamicRoadSystem/Blueprints/BP_RoadSystem.BP_RoadSystem_C|GetResolution%20Multiplier _array_element) (Variables|Baking|GetResolution%20Multiplier)))
        (Variables|/Game/Staging/DynamicRoadSystem/Blueprints/BP_RoadSystem.BP_RoadSystem_C|SetBakeToStaticMesh _array_element true)
        (Variables|/Game/Staging/DynamicRoadSystem/Blueprints/BP_RoadSystem.BP_RoadSystem_C|SetEnable%20Nanite _array_element (Variables|Baking|GetForce%20Nanite%20Enabled))
        (Default|ForceRebuild _array_element)
        (Variables|/Game/Staging/DynamicRoadSystem/Blueprints/BP_RoadSystem.BP_RoadSystem_C|SetResolution%20Multiplier _array_element (/ (Variables|/Game/Staging/DynamicRoadSystem/Blueprints/BP_RoadSystem.BP_RoadSystem_C|GetResolution%20Multiplier _array_element) (Variables|Baking|GetResolution%20Multiplier)))))
    (:then_1
      (bind _outactors_2 (Actor|GetAllActorsOfClass "/Game/Staging/DynamicRoadSystem/Blueprints/BP_RoadConnection.BP_RoadConnection_C"))
      (for _array_element_2 _outactors_2
        (Variables|/Game/Staging/DynamicRoadSystem/Blueprints/BP_RoadConnection.BP_RoadConnection_C|SetResolution%20Multiplier _array_element_2 (* (Variables|/Game/Staging/DynamicRoadSystem/Blueprints/BP_RoadConnection.BP_RoadConnection_C|GetResolution%20Multiplier _array_element_2) (Variables|Baking|GetResolution%20Multiplier)))
        (Variables|/Game/Staging/DynamicRoadSystem/Blueprints/BP_RoadConnection.BP_RoadConnection_C|SetBake%20To%20Static%20Mesh? _array_element_2 true)
        (Variables|/Game/Staging/DynamicRoadSystem/Blueprints/BP_RoadConnection.BP_RoadConnection_C|SetEnable%20Nanite _array_element_2 (Variables|Baking|GetForce%20Nanite%20Enabled))
        (Default|ForceRebuild _array_element_2)
        (Variables|/Game/Staging/DynamicRoadSystem/Blueprints/BP_RoadConnection.BP_RoadConnection_C|SetResolution%20Multiplier _array_element_2 (/ (Variables|/Game/Staging/DynamicRoadSystem/Blueprints/BP_RoadConnection.BP_RoadConnection_C|GetResolution%20Multiplier _array_element_2) (Variables|Baking|GetResolution%20Multiplier)))))
    (:then_2
      (bind _outactors_3 (Actor|GetAllActorsOfClass "/Game/Staging/DynamicRoadSystem/Blueprints/BP_RoadCrossingLot.BP_RoadCrossingLot_C"))
      (for _array_element_3 _outactors_3
        (Variables|/Game/Staging/DynamicRoadSystem/Blueprints/BP_RoadCrossingLot.BP_RoadCrossingLot_C|SetResolution%20Multiplier _array_element_3 (* (Variables|/Game/Staging/DynamicRoadSystem/Blueprints/BP_RoadCrossingLot.BP_RoadCrossingLot_C|GetResolution%20Multiplier _array_element_3) (Variables|Baking|GetResolution%20Multiplier)))
        (Variables|/Game/Staging/DynamicRoadSystem/Blueprints/BP_RoadCrossingLot.BP_RoadCrossingLot_C|SetBakeToStaticMesh _array_element_3 true)
        (Variables|/Game/Staging/DynamicRoadSystem/Blueprints/BP_RoadCrossingLot.BP_RoadCrossingLot_C|SetEnable%20Nanite _array_element_3 (Variables|Baking|GetForce%20Nanite%20Enabled))
        (Default|ForceRebuild _array_element_3)
        (Variables|/Game/Staging/DynamicRoadSystem/Blueprints/BP_RoadCrossingLot.BP_RoadCrossingLot_C|SetResolution%20Multiplier _array_element_3 (/ (Variables|/Game/Staging/DynamicRoadSystem/Blueprints/BP_RoadCrossingLot.BP_RoadCrossingLot_C|GetResolution%20Multiplier _array_element_3) (Variables|Baking|GetResolution%20Multiplier))))
      ;[1 1 1] debug amount of time for function
      (Development|PrintString (Utilities|String|Append "Baking took x milliseconds: " (Utilities|String|ToString(Integer) (+ (- (* (.minute _returnvalue) 60000) (* (.minute (LocalVariables|GetDebug%20Time)) 60000)) (- (* (.second _returnvalue) 1000) (* (.second (LocalVariables|GetDebug%20Time)) 1000)) (- (.millisecond _returnvalue) (.millisecond (LocalVariables|GetDebug%20Time)))))) false true "(R=0.000000,G=0.660000,B=1.000000,A=1.000000)" 5.0))))

(fn UpdateAllRoads
  (bind _returnvalue (Math|DateTime|Now))
  (bind _update_road_resolution (Variables|Debug|GetUpdate%20Road%20Resolution))
  (bind _update_road_resolution_2 (Variables|Debug|GetUpdate%20Road%20Resolution))
  (bind _update_road_resolution_3 (Variables|Debug|GetUpdate%20Road%20Resolution))
  ;[1 1 1] Debug time
  (LocalVariables|SetDebug%20Time (Math|DateTime|Now))
  (Utilities|FlowControl|Sequence
    (:then_0
      (bind _outactors (Actor|GetAllActorsOfClass "/Game/Staging/DynamicRoadSystem/Blueprints/BP_RoadSystem.BP_RoadSystem_C"))
      (for _array_element _outactors
        (if (== _update_road_resolution_2 0.0)
          _
          (else
            (Variables|/Game/Staging/DynamicRoadSystem/Blueprints/BP_RoadSystem.BP_RoadSystem_C|SetResolution%20Multiplier _array_element _update_road_resolution_2)))
        (Default|ForceRebuild _array_element)))
    (:then_1
      (bind _outactors_2 (Actor|GetAllActorsOfClass "/Game/Staging/DynamicRoadSystem/Blueprints/BP_RoadCrossingLot.BP_RoadCrossingLot_C"))
      (for _array_element_2 _outactors_2
        (if (== _update_road_resolution_3 0.0)
          _
          (else
            (Variables|/Game/Staging/DynamicRoadSystem/Blueprints/BP_RoadCrossingLot.BP_RoadCrossingLot_C|SetResolution%20Multiplier _array_element_2 _update_road_resolution_3)))
        (Default|ForceRebuild _array_element_2)))
    (:then_2
      (bind _outactors_3 (Actor|GetAllActorsOfClass "/Game/Staging/DynamicRoadSystem/Blueprints/BP_RoadConnection.BP_RoadConnection_C"))
      (for _array_element_3 _outactors_3
        (if (== _update_road_resolution 0.0)
          _
          (else
            (Variables|/Game/Staging/DynamicRoadSystem/Blueprints/BP_RoadConnection.BP_RoadConnection_C|SetResolution%20Multiplier _array_element_3 _update_road_resolution)))
        (Variables|/Game/Staging/DynamicRoadSystem/Blueprints/BP_RoadConnection.BP_RoadConnection_C|SetReset%20Connection _array_element_3 (Variables|Debug|GetReset%20Connections))
        (Default|ForceRebuild _array_element_3))
      (if (Variables|Debug|GetOSM%20Extend%20Lane%20Lines)
        (Debug|ExtendOSMLines)
        (Variables|Debug|SetOSM%20Extend%20Lane%20Lines false))
      ;[1 1 1] debug amount of time for function
      (Development|PrintString (Utilities|String|Append "Updating took x milliseconds: " (Utilities|String|ToString(Integer) (+ (- (* (.minute _returnvalue) 60000) (* (.minute (LocalVariables|GetDebug%20Time)) 60000)) (- (* (.second _returnvalue) 1000) (* (.second (LocalVariables|GetDebug%20Time)) 1000)) (- (.millisecond _returnvalue) (.millisecond (LocalVariables|GetDebug%20Time)))))) false true "(R=0.000000,G=0.660000,B=1.000000,A=1.000000)" 5.0))))

(fn ReportRoadOverlaps
  (bind _returnvalue (Math|DateTime|Now))
  ;[1 1 1] Debug time
  (LocalVariables|SetDebug%20Time (Math|DateTime|Now))
  (Utilities|FlowControl|Sequence
    (:then_0
      (bind _outactors (Actor|GetAllActorsOfClass "/Game/Staging/DynamicRoadSystem/Blueprints/BP_RoadSystem.BP_RoadSystem_C"))
      (for _array_element _outactors
        (Debug|TraceRoadsforConflicts (Variables|/Game/Staging/DynamicRoadSystem/Blueprints/BP_RoadSystem.BP_RoadSystem_C|GetRoadPoints _array_element) _array_element (Variables|/Game/Staging/DynamicRoadSystem/Blueprints/BP_RoadSystem.BP_RoadSystem_C|GetActors%20to%20Ignore%20when%20Snapping%20to%20Ground _array_element) _array_element)))
    (:then_1
      (bind _outactors_2 (Actor|GetAllActorsOfClass "/Game/Staging/DynamicRoadSystem/Blueprints/BP_RoadCrossingLot.BP_RoadCrossingLot_C"))
      (for _array_element_2 _outactors_2
        (Debug|TraceRoadsforConflicts (Variables|/Game/Staging/DynamicRoadSystem/Blueprints/BP_RoadCrossingLot.BP_RoadCrossingLot_C|GetRoadPoints _array_element_2) _array_element_2 (Variables|/Game/Staging/DynamicRoadSystem/Blueprints/BP_RoadCrossingLot.BP_RoadCrossingLot_C|GetActors%20to%20Ignore%20when%20Tracing _array_element_2) _array_element_2)))
    (:then_2
      (bind _outactors_3 (Actor|GetAllActorsOfClass "/Game/Staging/DynamicRoadSystem/Blueprints/BP_RoadConnection.BP_RoadConnection_C"))
      (for _array_element_3 _outactors_3
        (for (_array_element_4 _array_index) (Variables|/Game/Staging/DynamicRoadSystem/Blueprints/BP_RoadConnection.BP_RoadConnection_C|GetRoad%20Points _array_element_3)
          (Utilities|Array|SetArrayElem (LocalVariables|GetNew%20Road%20Point%20Array) _array_index (+ _array_element_4 (Transformation|GetActorLocation _array_element_3)) true))
        (Debug|TraceRoadsforConflicts (LocalVariables|GetNew%20Road%20Point%20Array) _array_element_3 (Variables|/Game/Staging/DynamicRoadSystem/Blueprints/BP_RoadConnection.BP_RoadConnection_C|GetActors%20to%20Ignore%20when%20Snapping%20to%20Ground _array_element_3) _array_element_3 (.connectedroad (Variables|/Game/Staging/DynamicRoadSystem/Blueprints/BP_RoadConnection.BP_RoadConnection_C|GetMainConnectedRoad _array_element_3)) (.connectedcrossinglot (Variables|/Game/Staging/DynamicRoadSystem/Blueprints/BP_RoadConnection.BP_RoadConnection_C|GetMainConnectedRoad _array_element_3)) (Variables|/Game/Staging/DynamicRoadSystem/Blueprints/BP_RoadConnection.BP_RoadConnection_C|GetSecondaryConnectedRoad _array_element_3))
        (Utilities|Array|Clear (LocalVariables|GetNew%20Road%20Point%20Array)))
      ;[1 1 1] debug amount of time for function
      (Development|PrintString (Utilities|String|Append "Updating took x milliseconds: " (Utilities|String|ToString(Integer) (+ (- (* (.minute _returnvalue) 60000) (* (.minute (LocalVariables|GetDebug%20Time)) 60000)) (- (* (.second _returnvalue) 1000) (* (.second (LocalVariables|GetDebug%20Time)) 1000)) (- (.millisecond _returnvalue) (.millisecond (LocalVariables|GetDebug%20Time)))))) false true "(R=0.000000,G=0.660000,B=1.000000,A=1.000000)" 5.0)
      (return))))

(fn TraceRoadsforConflicts
  (params (Road%20Points :type Array%20of%20Vectors) (Traced%20Road :type Object%20Object%20Reference) (Actors%20to%20Ignore%20%28Snapping%20to%20Ground%29 :type Array%20of%20Actor%20Object%20References) (Traced%20Road%20Actor :type Actor%20Object%20Reference%20%28by%20ref%29) (%28Optional%29%20Main%20Road :type BP%20Road%20System%20Object%20Reference) (%28Optional%29%20Crossing%20Lot :type BP%20Road%20Crossing%20Lot%20Object%20Reference) (%28Optional%29%20Secondary%20Road :type BP%20Road%20System%20Object%20Reference))
  (bind _output_get (LocalVariables|SetActors%20to%20Ignore Actors%20to%20Ignore%20%28Snapping%20to%20Ground%29))
  (if (Variables|Debug|GetAllow%20Road%20Overlap) ; if allow road overlap is false empty actors to ignore so it can print all overlapped roads
    _
    (else
      (Utilities|Array|Clear _output_get)))
  (Utilities|Array|AddUnique _output_get Traced%20Road%20Actor)
  (Utilities|Array|AddUnique _output_get %28Optional%29%20Main%20Road)
  (Utilities|Array|AddUnique _output_get %28Optional%29%20Crossing%20Lot)
  (Utilities|Array|AddUnique _output_get %28Optional%29%20Secondary%20Road)
  (for _array_element Road%20Points
    (bind (_outhit _returnvalue) (Collision|LineTraceByChannel (Math|Vector|MakeVector (.x _array_element) (.y _array_element) (+ (.z _array_element) 1e+03)) (Math|Vector|MakeVector (.x _array_element) (.y _array_element) (- (.z _array_element) 1e+03)) "TraceTypeQuery1" true (LocalVariables|GetActors%20to%20Ignore) "None" false "(R=1.000000,G=0.000000,B=0.000000,A=0.000000)" "(R=0.000000,G=1.000000,B=0.000000,A=1.000000)" 1e+01 :!label _label))
    (if _returnvalue
      (if (Math|Boolean|ORBoolean (== (Utilities|GetClass (.hitactor _outhit)) "/Game/Staging/DynamicRoadSystem/Blueprints/BP_RoadSystem.BP_RoadSystem_C") (== (Utilities|GetClass (.hitactor _outhit)) "/Game/Staging/DynamicRoadSystem/Blueprints/BP_RoadCrossingLot.BP_RoadCrossingLot_C") (and (== (Utilities|GetClass (.hitactor _outhit)) "/Game/Staging/DynamicRoadSystem/Blueprints/BP_RoadConnection.BP_RoadConnection_C") (== (Utilities|Array|FindItem Actors%20to%20Ignore%20%28Snapping%20to%20Ground%29 (.hitactor _outhit)) -1)))
        (Development|PrintString (Utilities|String|Append (Utilities|GetDisplayName Traced%20Road) " is overlapping " (Utilities|GetDisplayName (.hitactor _outhit))) false)
        (Utilities|Array|AddUnique (LocalVariables|GetActors%20to%20Ignore) (.hitactor _outhit))
        (if (Variables|Debug|GetAllow%20Road%20Overlap)
          (Utilities|Array|AddUnique Actors%20to%20Ignore%20%28Snapping%20to%20Ground%29 (.hitactor _outhit))
          (goto _label)))))
  (return))

(fn ExtendOSMLines
  (bind _returnvalue (Math|DateTime|Now))
  ;[1 1 1] Debug time
  (LocalVariables|SetDebug%20Time (Math|DateTime|Now))
  (bind _outactors (Actor|GetAllActorsOfClass "/Game/Staging/DynamicRoadSystem/Blueprints/BP_RoadSystem.BP_RoadSystem_C"))
  (for _array_element _outactors
    (for _array_element_2 (Variables|/Game/Staging/DynamicRoadSystem/Blueprints/BP_RoadSystem.BP_RoadSystem_C|GetRoad%20Connector _array_element)
      (if (.connecttoroadend? (Variables|/Game/Staging/DynamicRoadSystem/Blueprints/BP_RoadConnection.BP_RoadConnection_C|GetMainConnectedRoad _array_element_2))
        (if (and (== (.connectedroad (Variables|/Game/Staging/DynamicRoadSystem/Blueprints/BP_RoadConnection.BP_RoadConnection_C|GetMainConnectedRoad _array_element_2)) _array_element) (>= (Math|Vector|Distance(Vector) (Spline|GetLocationatSplinePoint (Variables|/Game/Staging/DynamicRoadSystem/Blueprints/BP_RoadConnection.BP_RoadConnection_C|GetMainSpline _array_element_2) 2 "World") (Spline|GetLocationatSplinePoint (Variables|/Game/Staging/DynamicRoadSystem/Blueprints/BP_RoadConnection.BP_RoadConnection_C|GetMainSpline _array_element_2) 12 "World")) (Math|Vector|Distance(Vector) (Spline|GetLocationatSplinePoint (Variables|/Game/Staging/DynamicRoadSystem/Blueprints/BP_RoadConnection.BP_RoadConnection_C|GetMainSpline _array_element_2) 14 "World") (Spline|GetLocationatSplinePoint (Variables|/Game/Staging/DynamicRoadSystem/Blueprints/BP_RoadConnection.BP_RoadConnection_C|GetMainSpline _array_element_2) 16 "World"))))
          (if (== (.pointofconnection (Variables|/Game/Staging/DynamicRoadSystem/Blueprints/BP_RoadConnection.BP_RoadConnection_C|GetMainConnectedRoad _array_element_2)) 0)
            (LocalVariables|SetNew%20Start%20Cutoff (* (Math|Vector|Distance(Vector) (Spline|GetLocationatSplinePoint (Variables|/Game/Staging/DynamicRoadSystem/Blueprints/BP_RoadConnection.BP_RoadConnection_C|GetMainSpline _array_element_2) 15 "World") (Spline|GetLocationatSplinePoint (Variables|/Game/Staging/DynamicRoadSystem/Blueprints/BP_RoadConnection.BP_RoadConnection_C|GetMainSpline _array_element_2) 7 "World")) -1.0))
            (else
              (LocalVariables|SetNew%20End%20Cutoff (* (Math|Vector|Distance(Vector) (Spline|GetLocationatSplinePoint (Variables|/Game/Staging/DynamicRoadSystem/Blueprints/BP_RoadConnection.BP_RoadConnection_C|GetMainSpline _array_element_2) 15 "World") (Spline|GetLocationatSplinePoint (Variables|/Game/Staging/DynamicRoadSystem/Blueprints/BP_RoadConnection.BP_RoadConnection_C|GetMainSpline _array_element_2) 7 "World")) -1.0))))
          (for _index (range 1 (- (Variables|/Game/Staging/DynamicRoadSystem/Blueprints/BP_RoadSystem.BP_RoadSystem_C|GetNumberOfLeftLanes _array_element) 1))
            (Utilities|Map|Add (Variables|/Game/Staging/DynamicRoadSystem/Blueprints/BP_RoadSystem.BP_RoadSystem_C|GetRoad%20Lines _array_element) (Utilities|String|Append "LeftLane_" (Utilities|String|ToString(Integer) _index)) (Utilities|Struct|MakeStruct_RoadLine (.Disable (Utilities|Struct|BreakStruct_RoadLine (.Value (Utilities|Map|Find (Variables|/Game/Staging/DynamicRoadSystem/Blueprints/BP_RoadSystem.BP_RoadSystem_C|GetRoad%20Lines _array_element) (Utilities|String|Append "LeftLane_" (Utilities|String|ToString(Integer) _index)))))) (.Shift (Utilities|Struct|BreakStruct_RoadLine (.Value (Utilities|Map|Find (Variables|/Game/Staging/DynamicRoadSystem/Blueprints/BP_RoadSystem.BP_RoadSystem_C|GetRoad%20Lines _array_element) (Utilities|String|Append "LeftLane_" (Utilities|String|ToString(Integer) _index)))))) (.Width (Utilities|Struct|BreakStruct_RoadLine (.Value (Utilities|Map|Find (Variables|/Game/Staging/DynamicRoadSystem/Blueprints/BP_RoadSystem.BP_RoadSystem_C|GetRoad%20Lines _array_element) (Utilities|String|Append "LeftLane_" (Utilities|String|ToString(Integer) _index)))))) (.MaterialID (Utilities|Struct|BreakStruct_RoadLine (.Value (Utilities|Map|Find (Variables|/Game/Staging/DynamicRoadSystem/Blueprints/BP_RoadSystem.BP_RoadSystem_C|GetRoad%20Lines _array_element) (Utilities|String|Append "LeftLane_" (Utilities|String|ToString(Integer) _index)))))) (LocalVariables|GetNew%20Start%20Cutoff) (LocalVariables|GetNew%20End%20Cutoff) (.DashedLineGapRatio (Utilities|Struct|BreakStruct_RoadLine (.Value (Utilities|Map|Find (Variables|/Game/Staging/DynamicRoadSystem/Blueprints/BP_RoadSystem.BP_RoadSystem_C|GetRoad%20Lines _array_element) (Utilities|String|Append "LeftLane_" (Utilities|String|ToString(Integer) _index)))))) (.DashedLineDistance (Utilities|Struct|BreakStruct_RoadLine (.Value (Utilities|Map|Find (Variables|/Game/Staging/DynamicRoadSystem/Blueprints/BP_RoadSystem.BP_RoadSystem_C|GetRoad%20Lines _array_element) (Utilities|String|Append "LeftLane_" (Utilities|String|ToString(Integer) _index)))))))))
          (for _index_2 (range 1 (- (Variables|/Game/Staging/DynamicRoadSystem/Blueprints/BP_RoadSystem.BP_RoadSystem_C|GetNumberOfRightLanes _array_element) 1))
            (Utilities|Map|Add (Variables|/Game/Staging/DynamicRoadSystem/Blueprints/BP_RoadSystem.BP_RoadSystem_C|GetRoad%20Lines _array_element) (Utilities|String|Append "RightLane_" (Utilities|String|ToString(Integer) _index_2)) (Utilities|Struct|MakeStruct_RoadLine (.Disable (Utilities|Struct|BreakStruct_RoadLine (.Value (Utilities|Map|Find (Variables|/Game/Staging/DynamicRoadSystem/Blueprints/BP_RoadSystem.BP_RoadSystem_C|GetRoad%20Lines _array_element) (Utilities|String|Append "RightLane_" (Utilities|String|ToString(Integer) _index_2)))))) (.Shift (Utilities|Struct|BreakStruct_RoadLine (.Value (Utilities|Map|Find (Variables|/Game/Staging/DynamicRoadSystem/Blueprints/BP_RoadSystem.BP_RoadSystem_C|GetRoad%20Lines _array_element) (Utilities|String|Append "RightLane_" (Utilities|String|ToString(Integer) _index_2)))))) (.Width (Utilities|Struct|BreakStruct_RoadLine (.Value (Utilities|Map|Find (Variables|/Game/Staging/DynamicRoadSystem/Blueprints/BP_RoadSystem.BP_RoadSystem_C|GetRoad%20Lines _array_element) (Utilities|String|Append "RightLane_" (Utilities|String|ToString(Integer) _index_2)))))) (.MaterialID (Utilities|Struct|BreakStruct_RoadLine (.Value (Utilities|Map|Find (Variables|/Game/Staging/DynamicRoadSystem/Blueprints/BP_RoadSystem.BP_RoadSystem_C|GetRoad%20Lines _array_element) (Utilities|String|Append "RightLane_" (Utilities|String|ToString(Integer) _index_2)))))) (LocalVariables|GetNew%20Start%20Cutoff) (LocalVariables|GetNew%20End%20Cutoff) (.DashedLineGapRatio (Utilities|Struct|BreakStruct_RoadLine (.Value (Utilities|Map|Find (Variables|/Game/Staging/DynamicRoadSystem/Blueprints/BP_RoadSystem.BP_RoadSystem_C|GetRoad%20Lines _array_element) (Utilities|String|Append "RightLane_" (Utilities|String|ToString(Integer) _index_2)))))) (.DashedLineDistance (Utilities|Struct|BreakStruct_RoadLine (.Value (Utilities|Map|Find (Variables|/Game/Staging/DynamicRoadSystem/Blueprints/BP_RoadSystem.BP_RoadSystem_C|GetRoad%20Lines _array_element) (Utilities|String|Append "RightLane_" (Utilities|String|ToString(Integer) _index_2)))))))))
          (LocalVariables|SetNew%20Start%20Cutoff 0.0)
          (LocalVariables|SetNew%20End%20Cutoff 0.0)
          (Default|ForceRebuild _array_element)
          (elif (and (not (>= (Math|Vector|Distance(Vector) (Spline|GetLocationatSplinePoint (Variables|/Game/Staging/DynamicRoadSystem/Blueprints/BP_RoadConnection.BP_RoadConnection_C|GetMainSpline _array_element_2) 2 "World") (Spline|GetLocationatSplinePoint (Variables|/Game/Staging/DynamicRoadSystem/Blueprints/BP_RoadConnection.BP_RoadConnection_C|GetMainSpline _array_element_2) 12 "World")) (Math|Vector|Distance(Vector) (Spline|GetLocationatSplinePoint (Variables|/Game/Staging/DynamicRoadSystem/Blueprints/BP_RoadConnection.BP_RoadConnection_C|GetMainSpline _array_element_2) 14 "World") (Spline|GetLocationatSplinePoint (Variables|/Game/Staging/DynamicRoadSystem/Blueprints/BP_RoadConnection.BP_RoadConnection_C|GetMainSpline _array_element_2) 16 "World")))) (== (Variables|/Game/Staging/DynamicRoadSystem/Blueprints/BP_RoadConnection.BP_RoadConnection_C|GetSecondaryConnectedRoad _array_element_2) _array_element))
            (if (Utilities|Enum|Equal(Enum) (Variables|/Game/Staging/DynamicRoadSystem/Blueprints/BP_RoadConnection.BP_RoadConnection_C|GetConnection%20Point _array_element_2) "NewEnumerator0")
              (LocalVariables|SetNew%20Start%20Cutoff (* (Math|Vector|Distance(Vector) (Spline|GetLocationatSplinePoint (Variables|/Game/Staging/DynamicRoadSystem/Blueprints/BP_RoadConnection.BP_RoadConnection_C|GetMainSpline _array_element_2) 15 "World") (Spline|GetLocationatSplinePoint (Variables|/Game/Staging/DynamicRoadSystem/Blueprints/BP_RoadConnection.BP_RoadConnection_C|GetMainSpline _array_element_2) 7 "World")) -1.0))
              (else
                (LocalVariables|SetNew%20End%20Cutoff (* (Math|Vector|Distance(Vector) (Spline|GetLocationatSplinePoint (Variables|/Game/Staging/DynamicRoadSystem/Blueprints/BP_RoadConnection.BP_RoadConnection_C|GetMainSpline _array_element_2) 15 "World") (Spline|GetLocationatSplinePoint (Variables|/Game/Staging/DynamicRoadSystem/Blueprints/BP_RoadConnection.BP_RoadConnection_C|GetMainSpline _array_element_2) 7 "World")) -1.0))))
            (for _index_3 (range 1 (- (Variables|/Game/Staging/DynamicRoadSystem/Blueprints/BP_RoadSystem.BP_RoadSystem_C|GetNumberOfLeftLanes _array_element) 1))
              (Utilities|Map|Add (Variables|/Game/Staging/DynamicRoadSystem/Blueprints/BP_RoadSystem.BP_RoadSystem_C|GetRoad%20Lines _array_element) (Utilities|String|Append "LeftLane_" (Utilities|String|ToString(Integer) _index_3)) (Utilities|Struct|MakeStruct_RoadLine (.Disable (Utilities|Struct|BreakStruct_RoadLine (.Value (Utilities|Map|Find (Variables|/Game/Staging/DynamicRoadSystem/Blueprints/BP_RoadSystem.BP_RoadSystem_C|GetRoad%20Lines _array_element) (Utilities|String|Append "LeftLane_" (Utilities|String|ToString(Integer) _index_3)))))) (.Shift (Utilities|Struct|BreakStruct_RoadLine (.Value (Utilities|Map|Find (Variables|/Game/Staging/DynamicRoadSystem/Blueprints/BP_RoadSystem.BP_RoadSystem_C|GetRoad%20Lines _array_element) (Utilities|String|Append "LeftLane_" (Utilities|String|ToString(Integer) _index_3)))))) (.Width (Utilities|Struct|BreakStruct_RoadLine (.Value (Utilities|Map|Find (Variables|/Game/Staging/DynamicRoadSystem/Blueprints/BP_RoadSystem.BP_RoadSystem_C|GetRoad%20Lines _array_element) (Utilities|String|Append "LeftLane_" (Utilities|String|ToString(Integer) _index_3)))))) (.MaterialID (Utilities|Struct|BreakStruct_RoadLine (.Value (Utilities|Map|Find (Variables|/Game/Staging/DynamicRoadSystem/Blueprints/BP_RoadSystem.BP_RoadSystem_C|GetRoad%20Lines _array_element) (Utilities|String|Append "LeftLane_" (Utilities|String|ToString(Integer) _index_3)))))) (LocalVariables|GetNew%20Start%20Cutoff) (LocalVariables|GetNew%20End%20Cutoff) (.DashedLineGapRatio (Utilities|Struct|BreakStruct_RoadLine (.Value (Utilities|Map|Find (Variables|/Game/Staging/DynamicRoadSystem/Blueprints/BP_RoadSystem.BP_RoadSystem_C|GetRoad%20Lines _array_element) (Utilities|String|Append "LeftLane_" (Utilities|String|ToString(Integer) _index_3)))))) (.DashedLineDistance (Utilities|Struct|BreakStruct_RoadLine (.Value (Utilities|Map|Find (Variables|/Game/Staging/DynamicRoadSystem/Blueprints/BP_RoadSystem.BP_RoadSystem_C|GetRoad%20Lines _array_element) (Utilities|String|Append "LeftLane_" (Utilities|String|ToString(Integer) _index_3)))))))))
            (for _index_4 (range 1 (- (Variables|/Game/Staging/DynamicRoadSystem/Blueprints/BP_RoadSystem.BP_RoadSystem_C|GetNumberOfRightLanes _array_element) 1))
              (Utilities|Map|Add (Variables|/Game/Staging/DynamicRoadSystem/Blueprints/BP_RoadSystem.BP_RoadSystem_C|GetRoad%20Lines _array_element) (Utilities|String|Append "RightLane_" (Utilities|String|ToString(Integer) _index_4)) (Utilities|Struct|MakeStruct_RoadLine (.Disable (Utilities|Struct|BreakStruct_RoadLine (.Value (Utilities|Map|Find (Variables|/Game/Staging/DynamicRoadSystem/Blueprints/BP_RoadSystem.BP_RoadSystem_C|GetRoad%20Lines _array_element) (Utilities|String|Append "RightLane_" (Utilities|String|ToString(Integer) _index_4)))))) (.Shift (Utilities|Struct|BreakStruct_RoadLine (.Value (Utilities|Map|Find (Variables|/Game/Staging/DynamicRoadSystem/Blueprints/BP_RoadSystem.BP_RoadSystem_C|GetRoad%20Lines _array_element) (Utilities|String|Append "RightLane_" (Utilities|String|ToString(Integer) _index_4)))))) (.Width (Utilities|Struct|BreakStruct_RoadLine (.Value (Utilities|Map|Find (Variables|/Game/Staging/DynamicRoadSystem/Blueprints/BP_RoadSystem.BP_RoadSystem_C|GetRoad%20Lines _array_element) (Utilities|String|Append "RightLane_" (Utilities|String|ToString(Integer) _index_4)))))) (.MaterialID (Utilities|Struct|BreakStruct_RoadLine (.Value (Utilities|Map|Find (Variables|/Game/Staging/DynamicRoadSystem/Blueprints/BP_RoadSystem.BP_RoadSystem_C|GetRoad%20Lines _array_element) (Utilities|String|Append "RightLane_" (Utilities|String|ToString(Integer) _index_4)))))) (LocalVariables|GetNew%20Start%20Cutoff) (LocalVariables|GetNew%20End%20Cutoff) (.DashedLineGapRatio (Utilities|Struct|BreakStruct_RoadLine (.Value (Utilities|Map|Find (Variables|/Game/Staging/DynamicRoadSystem/Blueprints/BP_RoadSystem.BP_RoadSystem_C|GetRoad%20Lines _array_element) (Utilities|String|Append "RightLane_" (Utilities|String|ToString(Integer) _index_4)))))) (.DashedLineDistance (Utilities|Struct|BreakStruct_RoadLine (.Value (Utilities|Map|Find (Variables|/Game/Staging/DynamicRoadSystem/Blueprints/BP_RoadSystem.BP_RoadSystem_C|GetRoad%20Lines _array_element) (Utilities|String|Append "RightLane_" (Utilities|String|ToString(Integer) _index_4)))))))))
            (LocalVariables|SetNew%20Start%20Cutoff 0.0)
            (LocalVariables|SetNew%20End%20Cutoff 0.0)
            (Default|ForceRebuild _array_element))))))
  ;[1 1 1] debug amount of time for function
  (Development|PrintString (Utilities|String|Append "Updating took x milliseconds: " (Utilities|String|ToString(Integer) (+ (- (* (.minute _returnvalue) 60000) (* (.minute (LocalVariables|GetDebug%20Time)) 60000)) (- (* (.second _returnvalue) 1000) (* (.second (LocalVariables|GetDebug%20Time)) 1000)) (- (.millisecond _returnvalue) (.millisecond (LocalVariables|GetDebug%20Time)))))) false true "(R=0.000000,G=0.660000,B=1.000000,A=1.000000)" 5.0)
  (return))