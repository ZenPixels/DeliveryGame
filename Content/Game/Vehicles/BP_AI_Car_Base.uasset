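; BP_AI_Car_Base is a base Blueprint for AI cars built on Chaos wheeled vehicle movement.
; BeginPlay caches the movement component and applies fixed steering and throttle inputs, with no navigation logic driving them.
; Tick switches the mesh's angular damping by ground contact, damping rotation only while airborne.
; The GetPath function and construction script are empty stubs.
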(event EventTick
  (params (DeltaSeconds :type Float%20%28single-precision%29))
  (Class|PrimitiveComponent|SetAngularDamping (Variables|Character|GetMesh) (Math|Float|SelectFloat 0.0 3.0 (AI|Components|NavMovement|IsMovingonGround (Variables|Default|GetChaos%20Wheeled%20Vehicle%20Movement%20Component)))) ; Damps rotation when in air
)

(event EventBeginPlay
  ;[1 1 1] Movement component setup
  (Utilities|FlowControl|Sequence
    (:then_0
      (bind _aschaos_wheeled_vehicle_movement_component (Utilities|Casting|CastToChaosWheeledVehicleMovementComponent (Variables|Default|GetVehicleMovementComponent)))
      (Variables|Default|SetChaos%20Wheeled%20Vehicle%20Movement%20Component _aschaos_wheeled_vehicle_movement_component))
    (:then_1
      (Class|ChaosVehicleMovementComponent|SetSteeringInput (Variables|Default|GetVehicleMovementComponent) 5.0))
    (:then_2
      (Class|ChaosVehicleMovementComponent|SetThrottleInput (Variables|Default|GetVehicleMovementComponent) 5e+01))))

(fn ConstructionScript)

(fn GetPath)