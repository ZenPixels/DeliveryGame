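; Modular character assembled from separate skeletal mesh parts that can be knocked dead by a hard impact.
; The construction script makes the Shoes, LowerBody, Hat and Head parts follow the main Mesh as leader pose.
; A strong hit on a living character sets IsDead on itself and its AI blackboard, starts ragdoll physics with the impact force, and plays a car thump.
; Any other hit sets movement velocity along the hit normal.
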(event EventBeginPlay)

(event Collision|EventActorBeginOverlap
  (params (OtherActor :type Actor%20Object%20Reference)))

(event EventTick
  (params (DeltaSeconds :type Float%20%28single-precision%29)))

(event Collision|EventHit
  (params (MyComp :type Primitive%20Component%20Object%20Reference) (Other :type Actor%20Object%20Reference) (OtherComp :type Primitive%20Component%20Object%20Reference) (bSelfMoved :type Boolean) (HitLocation :type Vector :default "0, 0, 0") (HitNormal :type Vector :default "0, 0, 0") (NormalImpulse :type Vector :default "0, 0, 0") (Hit :type Hit%20Result%20Structure%20%28by%20ref%29))
  (bind _mesh (Variables|Character|GetMesh))
  (if (and (> (Math|Vector|VectorLength NormalImpulse) 1e+02) (not (Variables|Default|GetIs%20Dead)))
    (Variables|Default|SetIs%20Dead true)
    (AI|Components|Blackboard|SetValueasBool (AI|GetBlackboard 0) (Utilities|Name|MakeLiteralName "IsDead") true)
    (Physics|SetSimulatePhysics _mesh true)
    (Physics|AddForce _mesh NormalImpulse "None" false)
    (Audio|PlaySoundatLocation "/Game/Vehicles/Veh_Offroad/Car_Thump.Car_Thump" HitLocation "0, 0, 0" 1.0 1.0 0.0 0 0 0 0)
    (else
      (Variables|/Script/Engine.MovementComponent|SetVelocity (Variables|Character|GetCharacterMovement) (* HitNormal 1.5)))))

(fn ConstructionScript
  (Components|SkinnedMesh|SetLeaderPoseComponent (Variables|Default|GetShoes) (Variables|Character|GetMesh) false false))