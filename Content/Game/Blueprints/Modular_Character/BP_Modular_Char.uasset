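; Modular AI character that randomizes its look on BeginPlay and ragdolls when struck hard, with a car thump sound.
; Weighted rolls pick skin and hair materials, then upper body, clothing colors, shoes, hat or hair, and head.
; Body parts follow the main Mesh through leader pose.
; A strong hit sets IsDead on the Blackboard and swaps capsule collision for mesh physics; other hits set velocity along the hit normal.
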(event EventBeginPlay
  (CallFunction|AssignSkinHairMaterial)
  (CallFunction|AssignUpperBody)
  (CallFunction|AssignShoes)
  (CallFunction|AssignHatHair)
  (CallFunction|AssignHead))

(event Collision|EventActorBeginOverlap
  (params (OtherActor :type Actor%20Object%20Reference)))

(event EventTick
  (params (DeltaSeconds :type Float%20%28single-precision%29)))

(event Collision|EventHit
  (params (MyComp :type Primitive%20Component%20Object%20Reference) (Other :type Actor%20Object%20Reference) (OtherComp :type Primitive%20Component%20Object%20Reference) (bSelfMoved :type Boolean) (HitLocation :type Vector :default "0, 0, 0") (HitNormal :type Vector :default "0, 0, 0") (NormalImpulse :type Vector :default "0, 0, 0") (Hit :type Hit%20Result%20Structure%20%28by%20ref%29))
  (bind _mesh (Variables|Character|GetMesh))
  (bind _capsulecomponent (Variables|Collision|GetCapsuleComponent))
  (if (and (> (Math|Vector|VectorLength NormalImpulse) 1e+02) (not (Variables|Default|GetIs%20Dead)))
    (Variables|Default|SetIs%20Dead true)
    (AI|Components|Blackboard|SetValueasBool (AI|GetBlackboard 0) (Utilities|Name|MakeLiteralName "IsDead") true)
    (Physics|SetSimulatePhysics _capsulecomponent false)
    (Collision|SetCollisionEnabled _capsulecomponent "NoCollision")
    (Physics|SetSimulatePhysics _mesh true)
    (Collision|SetCollisionEnabled _mesh "PhysicsOnly")
    (Physics|AddForce _mesh NormalImpulse "None" false)
    (Audio|PlaySoundatLocation "/Game/Game/Blueprints/Vehicle_Base/Collisions/Car_Thump.Car_Thump" HitLocation "0, 0, 0" 1.0 1.0 0.0 0 0 0 0)
    (else
      (Variables|/Script/Engine.MovementComponent|SetVelocity (Variables|Character|GetCharacterMovement) (* HitNormal 1.5)))))

(fn ConstructionScript
  (Components|SkinnedMesh|SetLeaderPoseComponent (Variables|Default|GetShoes) (Variables|Character|GetMesh) false false))

(fn AssignUpperBody
  (bind _mesh (Variables|Character|GetMesh))
  (bind _mesh_2 (Variables|Character|GetMesh))
  (bind _mesh_3 (Variables|Character|GetMesh))
  (bind _output_get (Variables|Default|SetRandom (Math|Random|RandomIntegerinRange 0 100)))
  (if (<= _output_get 70)
    (Components|SkeletalMesh|SetSkeletalMeshAsset _mesh_3 "/Game/Game/Meshes/Characters/Modular/UpperBody_Shirt_M_2.UpperBody_Shirt_M_2")
    (Rendering|Material|SetMaterialbyName (Variables|Character|GetMesh) "Skin" (Variables|Default|GetMaterial%20Skin) :!label _label)
    (bind _output_get_2 (Variables|Default|SetRandom (Math|Random|RandomIntegerinRange 0 100)))
    (if (<= _output_get_2 15)
      (Rendering|Material|SetMaterialbyName _mesh "Jacket" "/Game/Game/Materials/MI_Green_Dark.MI_Green_Dark")
      (bind _output_get_3 (Variables|Default|SetRandom (Math|Random|RandomIntegerinRange 0 100) :!label _label_2))
      (if (<= _output_get_3 15)
        (Rendering|Material|SetMaterialbyName _mesh_2 "Shirt" "/Game/Game/Materials/MI_Green_Dark.MI_Green_Dark")
        (elif (<= _output_get_3 30)
          (Rendering|Material|SetMaterialbyName _mesh_2 "Shirt" "/Game/Game/Materials/MI_Blue_Dark.MI_Blue_Dark")
          (elif (<= _output_get_3 45)
            (Rendering|Material|SetMaterialbyName _mesh_2 "Shirt" "/Game/Game/Materials/MI_Red_Dark.MI_Red_Dark")
            (elif (<= _output_get_3 60)
              (Rendering|Material|SetMaterialbyName _mesh_2 "Shirt" "/Game/Game/Materials/MI_Blue_Light.MI_Blue_Light")
              (elif (<= _output_get_3 75)
                (Rendering|Material|SetMaterialbyName _mesh_2 "Shirt" "/Game/Game/Materials/MI_Green_Light.MI_Green_Light")
                (elif (<= _output_get_3 85)
                  (Rendering|Material|SetMaterialbyName _mesh_2 "Shirt" "/Game/Game/Materials/MI_Orange_Red_Light.MI_Orange_Red_Light")
                  (elif (<= _output_get_3 100)
                    (Rendering|Material|SetMaterialbyName _mesh_2 "Shirt" "/Game/Game/Materials/MI_Black.MI_Black"))))))))
      (elif (<= _output_get_2 30)
        (Rendering|Material|SetMaterialbyName _mesh "Jacket" "/Game/Game/Materials/MI_Blue_Dark.MI_Blue_Dark")
        (goto _label_2)
        (elif (<= _output_get_2 45)
          (Rendering|Material|SetMaterialbyName _mesh "Jacket" "/Game/Game/Materials/MI_Red_Dark.MI_Red_Dark")
          (goto _label_2)
          (elif (<= _output_get_2 60)
            (Rendering|Material|SetMaterialbyName _mesh "Jacket" "/Game/Game/Materials/MI_Blue_Light.MI_Blue_Light")
            (goto _label_2)
            (elif (<= _output_get_2 75)
              (Rendering|Material|SetMaterialbyName _mesh "Jacket" "/Game/Game/Materials/MI_Green_Light.MI_Green_Light")
              (goto _label_2)
              (elif (<= _output_get_2 85)
                (Rendering|Material|SetMaterialbyName _mesh "Jacket" "/Game/Game/Materials/MI_Orange_Red_Light.MI_Orange_Red_Light")
                (goto _label_2)
                (elif (<= _output_get_2 100)
                  (Rendering|Material|SetMaterialbyName _mesh "Jacket" "/Game/Game/Materials/MI_Black.MI_Black")
                  (goto _label_2))))))))
    (elif (<= 85 _output_get)
      (Components|SkeletalMesh|SetSkeletalMeshAsset _mesh_3 "/Game/Game/Meshes/Characters/Modular/UpperBody_Jacket_M_1.UpperBody_Jacket_M_1")
      (goto _label)
      (elif (<= _output_get 95)
        (Components|SkeletalMesh|SetSkeletalMeshAsset _mesh_3 "/Game/Game/Meshes/Characters/Modular/UpperBody_Jacket_M_2.UpperBody_Jacket_M_2")
        (goto _label)
        (elif (<= _output_get 100)
          (Components|SkeletalMesh|SetSkeletalMeshAsset _mesh_3 "/Game/Game/Meshes/Characters/Modular/UpperBody_Shirt_M_1.UpperBody_Shirt_M_1")
          (goto _label))))))

(fn AssignShoes
  (bind _shoes (Variables|Default|GetShoes))
  (bind _output_get (Variables|Default|SetRandom (Math|Random|RandomIntegerinRange 0 100)))
  (if (<= _output_get 50)
    (Components|SkeletalMesh|SetSkeletalMeshAsset _shoes "/Game/Game/Meshes/Characters/Modular/Feet_Shoes_1.Feet_Shoes_1")
    (elif (<= _output_get 100)
      (Components|SkeletalMesh|SetSkeletalMeshAsset _shoes "/Game/Game/Meshes/Characters/Modular/Feet_Shoes_2.Feet_Shoes_2")
      (else
        (Components|SkeletalMesh|SetSkeletalMeshAsset _shoes "/Game/Game/Meshes/Characters/Modular/Feet_Shoes_1.Feet_Shoes_1")))))

(fn AssignHatHair
  (bind _hair (Variables|Default|GetHair))
  (bind _output_get (Variables|Default|SetRandom (Math|Random|RandomIntegerinRange 0 100)))
  (if (<= _output_get 6)
    (Components|SkeletalMesh|SetSkeletalMeshAsset _hair "/Game/Game/Meshes/Characters/Modular/Hat_M_1.Hat_M_1")
    (Rendering|Material|SetMaterialbyName (Variables|Default|GetHair) "Hair" (Variables|Default|GetMaterial%20Hair) :!label _label)
    (elif (<= _output_get 53)
      (Components|SkeletalMesh|SetSkeletalMeshAsset _hair "/Game/Game/Meshes/Characters/Modular/Hair/Hair_M_1.Hair_M_1")
      (goto _label)
      (elif (<= _output_get 100)
        (Components|SkeletalMesh|SetSkeletalMeshAsset _hair "/Game/Game/Meshes/Characters/Modular/Hair/Hair_M_2.Hair_M_2")
        (goto _label)))))

(fn AssignSkinHairMaterial
  (bind _output_get (Variables|Default|SetRandom (Math|Random|RandomIntegerinRange 0 100)))
  (if (<= _output_get 32)
    (Variables|Default|SetMaterial%20Skin "/Game/Game/Materials/MI_Peach_Light.MI_Peach_Light")
    (bind _output_get_2 (Variables|Default|SetRandom (Math|Random|RandomIntegerinRange 0 100) :!label _label))
    (if (<= _output_get_2 35)
      (Variables|Default|SetMaterial%20Hair "/Game/Game/Materials/MI_Black.MI_Black")
      (elif (<= _output_get_2 70)
        (Variables|Default|SetMaterial%20Hair "/Game/Game/Materials/MI_Brown_Dark.MI_Brown_Dark")
        (elif (<= _output_get_2 80)
          (Variables|Default|SetMaterial%20Hair "/Game/Game/Materials/MI_Brown_Light.MI_Brown_Light")
          (elif (<= _output_get_2 90)
            (Variables|Default|SetMaterial%20Hair "/Game/Game/Materials/MI_Brown_Med_1.MI_Brown_Med_1")
            (elif (<= _output_get_2 96)
              (Variables|Default|SetMaterial%20Hair "/Game/Game/Materials/MI_Yellow_Light.MI_Yellow_Light")
              (elif (<= _output_get_2 100)
                (Variables|Default|SetMaterial%20Hair "/Game/Game/Materials/MI_Orange_Red.MI_Orange_Red")))))))
    (elif (<= 64 _output_get)
      (Variables|Default|SetMaterial%20Skin "/Game/Game/Materials/MI_Peach_Med.MI_Peach_Med")
      (goto _label)
      (elif (<= _output_get 87)
        (Variables|Default|SetMaterial%20Skin "/Game/Game/Materials/MI_Brown_Med_2.MI_Brown_Med_2")
        (bind _output_get_3 (Variables|Default|SetRandom (Math|Random|RandomIntegerinRange 0 100) :!label _label_2))
        (if (<= _output_get_3 50)
          (Variables|Default|SetMaterial%20Hair "/Game/Game/Materials/MI_Black.MI_Black")
          (else
            (Variables|Default|SetMaterial%20Hair "/Game/Game/Materials/MI_Brown_Dark.MI_Brown_Dark")))
        (elif (<= _output_get 100)
          (Variables|Default|SetMaterial%20Skin "/Game/Game/Materials/MI_Orange_Yellow.MI_Orange_Yellow")
          (goto _label_2))))))

(fn AssignHead
  (bind _head (Variables|Default|GetHead))
  (bind _output_get (Variables|Default|SetRandom (Math|Random|RandomIntegerinRange 0 100)))
  (if (<= _output_get 50)
    (Components|SkeletalMesh|SetSkeletalMeshAsset _head "/Game/Game/Meshes/Characters/Modular/Head_M_1.Head_M_1")
    (Rendering|Material|SetMaterialbyName (Variables|Default|GetHead) "Hair" (Variables|Default|GetMaterial%20Hair) :!label _label)
    (Rendering|Material|SetMaterialbyName (Variables|Default|GetHead) "Skin" (Variables|Default|GetMaterial%20Skin))
    (elif (<= _output_get 100)
      (Components|SkeletalMesh|SetSkeletalMeshAsset _head "/Game/Game/Meshes/Characters/Modular/Head_M_2.Head_M_2")
      (goto _label))))