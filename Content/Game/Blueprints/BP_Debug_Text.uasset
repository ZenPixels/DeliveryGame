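; BP_Debug_Text is a debug component that displays strings in floating white text above its owning actor.
; BeginPlay adds a TextRenderComponent to the owner with a raised Z offset.
; Each Tick loops over the DebugStrings map keys, writes values to the text and turns it against the player controller's forward vector.
; The map and output buffer are cleared inside that loop, so entries do not accumulate.
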(event EventBeginPlay
  (bind _returnvalue (Game|AddComponentbyClass (Components|GetOwner) "/Script/Engine.TextRenderComponent" false (Math|Transform|MakeTransform (Math|Vector|MakeVector 0.0 0.0 (Math|Float|MakeLiteralFloat 275.0)) "0, 0, 0" "1.000000,1.000000,1.000000")))
  (bind _output_get (Variables|Default|SetDebug%20Text _returnvalue))
  (Rendering|Components|TextRender|SetTextRenderColor _output_get (Math|Color|MakeColor 1 1 1 1)))

(event EventTick
  (params (DeltaSeconds :type Float%20%28single-precision%29))
  (CallFunction|UpdateDebugText))

(fn UpdateDebugText
  (bind _debug_strings (Variables|Default|GetDebug%20Strings))
  (bind _keys (Utilities|Map|Keys _debug_strings))
  (for _array_element _keys
    (bind _output_get (Variables|Default|SetOutput%20Text (Utilities|String|Append (Variables|Default|GetOutput%20Text) (.Value (Utilities|Map|Find _debug_strings _array_element)) "<br>")))
    (Rendering|Components|TextRender|SetText (Variables|Default|GetDebug%20Text) (Utilities|Text|ToText(String) _output_get))
    (Transformation|SetWorldRotation (Variables|Default|GetDebug%20Text) (Math|Conversions|RotationFromXVector (Math|Rotator|GetRotationXVector (* (Transformation|GetActorForwardVector (Game|GetPlayerController 0)) -1.0))) false false)
    (CallFunction|ClearDebugText)))

(fn ClearDebugText
  (Utilities|Map|Clear (Variables|Default|GetDebug%20Strings))
  (Variables|Default|SetOutput%20Text ""))