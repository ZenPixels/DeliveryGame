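; Small traffic light prop that endlessly cycles green, yellow and red after an initial delay.
; A looping Delay chain on BeginPlay toggles the three light components' visibility and records the phase in CurrentLightState.
; SlowZone overlap events switch off for green and back on at yellow, staying on through red.
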(event EventBeginPlay
  (bind _slow_zone (Variables|Default|GetSlow%20Zone))
  (Utilities|FlowControl|Delay (Variables|Default|GetInit%20Delay))
  ;[1 1 1] Red -> Green (0 -> 2)
  (Rendering|SetVisibility (Variables|Default|GetRed%20Light) false false :!label _label)
  (Rendering|SetVisibility (Variables|Default|GetGreen%20Light) true false)
  (Variables|Default|SetCurrent%20Light%20State 2)
  (Variables|/Script/Engine.PrimitiveComponent|SetbGenerateOverlapEvents _slow_zone false)
  (Utilities|FlowControl|Delay (Variables|Default|GetGreen%20Time))
  ;[1 1 1] Green -> Yellow (2 -> 1)
  (Rendering|SetVisibility (Variables|Default|GetGreen%20Light) false false)
  (Rendering|SetVisibility (Variables|Default|GetYelllow%20Light) true false)
  (Variables|Default|SetCurrent%20Light%20State 1)
  (Variables|/Script/Engine.PrimitiveComponent|SetbGenerateOverlapEvents _slow_zone true)
  (Utilities|FlowControl|Delay (Variables|Default|GetYellow%20Time))
  ;[1 1 1] Yellow -> Red (1 -> 0)
  (Rendering|SetVisibility (Variables|Default|GetYelllow%20Light) false false)
  (Rendering|SetVisibility (Variables|Default|GetRed%20Light) true false)
  (Variables|Default|SetCurrent%20Light%20State 0)
  (Utilities|FlowControl|Delay (Variables|Default|GetRed%20Time))
  (goto _label))

(fn ConstructionScript)