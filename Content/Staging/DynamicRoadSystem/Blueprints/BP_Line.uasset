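; BP_Line is a spline-driven generated mesh actor that builds solid or dashed line markings for the dynamic road system.
; On rebuild, it optionally subdivides or reverts spline points, then snaps them to the ground with line traces unless disabled.
; It sweeps a rectangular profile along the spline, using a temporary spline for each dash when GapRatio is not 1.
; A separate function bakes the mesh to a per-level static mesh asset.
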(event Events|EventOnRebuildGeneratedMesh
  (params (TargetMesh :type Dynamic%20Mesh%20Object%20Reference))
  (bind _returnvalue (Math|DateTime|Now))
  (bind _line_distance_ (Variables|LineOptions|GetLine%20Distance%20))
  (bind _gap_ratio (Variables|LineOptions|GetGap%20Ratio))
  (bind _line_height (Variables|LineOptions|GetLine%20Height))
  (bind _line_width (Variables|LineOptions|GetLine%20Width))
  (bind _line_width_2 (Variables|LineOptions|GetLine%20Width))
  (bind _line_height_2 (Variables|LineOptions|GetLine%20Height))
  (bind _returnvalue_2 (Math|Conversions|ToFloat(Integer) _line_distance_))
  (bind _returnvalue_3 (- 1.0 _gap_ratio))
  (bind _returnvalue_4 (/ _line_width 2.0))
  (bind _returnvalue_5 (* _line_height -2.0))
  (bind _returnvalue_6 (/ _line_width_2 2.0))
  (bind _returnvalue_7 (* _line_height_2 -2.0))
  (bind _returnvalue_8 (* _returnvalue_2 _returnvalue_3))
  (bind _returnvalue_9 (* _returnvalue_4 -1.0))
  (bind _returnvalue_10 (* _returnvalue_6 -1.0))
  (bind _returnvalue_11 (Math|Float|Round _returnvalue_8))
  ;[1 1 1] Set initial variables
  (bind _returnvalue_12 (DynamicMesh|Reset TargetMesh))
  (Variables|Default|SetTarget%20Mesh _returnvalue_12)
  (if (Variables|LineOptions|GetShow%20Function%20Completion%20Time)
    (Variables|Default|SetDebugTime (Math|DateTime|Now)))
  ;[1 1 1] Subdivide or unsubdivide spline for better quality or better rendering time (respectively)
  (if (Variables|Actions|GetSubdivide%20Spline?)
    (bind _spline_points_out (CallFunction|SubdividePoints))
    (Spline|SetSplinePoints (Variables|Default|GetSpline) _spline_points_out "World" true)
    (Variables|Actions|SetSubdivide%20Spline? false)
    (elif (Variables|Actions|GetRevert%20Subdivision?)
      (bind _spline_points_out_2 (CallFunction|UnsubdividePoints))
      (Spline|SetSplinePoints (Variables|Default|GetSpline) _spline_points_out_2 "World" true)
      (Variables|Actions|SetRevert%20Subdivision? false)))
  (if (Variables|LineOptions|GetDisable%20Ground%20Snapping)
    _
    (else
      (CallFunction|SnaptoGround)))
  (if (== (Variables|LineOptions|GetGap%20Ratio) 1.0)
    ;[1 1 1 0.1] Create non-dashed line
    (bind _frames (Class|GeometryScriptLibraryPolyPathFunctions|SampleSplinetoTransforms :Spline (Variables|Default|GetSpline) :SamplingOptions (Utilities|Struct|MakeGeometryScriptSplineSamplingOptions (Math|Float|Truncate (/ (Spline|GetSplineLength (Variables|Default|GetSpline)) 1e+01)) 1.0 "UniformTime" "Local")))
    (Class|GeometryScriptLibraryMeshPrimitiveFunctions|AppendSweepPolygon :TargetMesh (Variables|Default|GetTarget%20Mesh) :PolygonVertices (Utilities|Array|MakeArray (Math|Vector2D|MakeVector2D _returnvalue_9 _returnvalue_5) (Math|Vector2D|MakeVector2D _returnvalue_4 _returnvalue_5) (Math|Vector2D|MakeVector2D _returnvalue_4 _line_height) (Math|Vector2D|MakeVector2D _returnvalue_9 _line_height)) :SweepPath _frames :Debug 0)
    (else
      ;[1 1 1 0.1] Create Dashed Line
      ;;[1 1 1 0.4] Create a spline that follows a portion of the road line
      (bind _returnvalue_13 (AddComponent|AddSplineComponent false))
      (Spline|ClearSplinePoints _returnvalue_13 true)
      (for _index (range 0 (- (/ (Math|Float|Round (Spline|GetSplineLength (Variables|Default|GetSpline))) _line_distance_) 1))
        (for _index_2 (range 0 4) ; 4 is the number of spline samples for each dashed road line (0-4 is technically 5 samples though)
          (Spline|AddSplinePoint _returnvalue_13 (Spline|GetLocationatDistanceAlongSpline (Variables|Default|GetSpline) (+ (Math|Conversions|ToFloat(Integer) (+ (* _index _line_distance_) _returnvalue_11)) (* (Math|Conversions|ToFloat(Integer) _index_2) (/ (- (Math|Conversions|ToFloat(Integer) (+ (+ (* _index _line_distance_) _returnvalue_11) (- _line_distance_ _returnvalue_11))) (Math|Conversions|ToFloat(Integer) (+ (* _index _line_distance_) _returnvalue_11))) 4.0))) "World") "World" false))
        ;;[1 1 1 0.4] Use the spline created above to subtract geometry from the main roads white lines
        (Spline|UpdateSpline _returnvalue_13)
        (bind _frames_2 (Class|GeometryScriptLibraryPolyPathFunctions|SampleSplinetoTransforms :Spline _returnvalue_13 :SamplingOptions (Utilities|Struct|MakeGeometryScriptSplineSamplingOptions 5 1.0 "UniformTime" "Local")))
        (Class|GeometryScriptLibraryMeshPrimitiveFunctions|AppendSweepPolygon :TargetMesh (Variables|Default|GetTarget%20Mesh) :PolygonVertices (Utilities|Array|MakeArray (Math|Vector2D|MakeVector2D _returnvalue_10 _returnvalue_7) (Math|Vector2D|MakeVector2D _returnvalue_6 _returnvalue_7) (Math|Vector2D|MakeVector2D _returnvalue_6 _line_height_2) (Math|Vector2D|MakeVector2D _returnvalue_10 _line_height_2)) :SweepPath _frames_2 :Debug 0)
        (Spline|ClearSplinePoints _returnvalue_13 true)
        (Class|DynamicMeshActor|ReleaseComputeMesh))
      (Components|DestroyComponent _returnvalue_13)
      (DynamicMeshActor|ReleaseAllComputeMeshes)))
  ;[1 1 1] debug amount of time for function
  (if (Variables|LineOptions|GetShow%20Function%20Completion%20Time)
    (Development|PrintString (Utilities|String|Append "Function took x milliseconds: " (Utilities|String|ToString(Integer) (+ (- (* (.minute _returnvalue) 60000) (* (.minute (Variables|Default|GetDebugTime)) 60000)) (- (* (.second _returnvalue) 1000) (* (.second (Variables|Default|GetDebugTime)) 1000)) (- (.millisecond _returnvalue) (.millisecond (Variables|Default|GetDebugTime)))))))))

(fn ConstructionScript)

(fn SubdividePoints
  (bind _spline (Variables|Default|GetSpline))
  (bind _temp_spline_points (LocalVariables|GetTemp%20Spline%20Points))
  (Utilities|Array|Clear (LocalVariables|GetTemp%20Spline%20Points))
  (for _index (range 0 (- (Spline|GetNumberOfSplinePoints (Variables|Default|GetSpline)) 1))
    (Utilities|Array|Add (LocalVariables|GetSpline%20Points) (Spline|GetLocationatSplinePoint (Variables|Default|GetSpline) _index "World")))
  (for (_array_element _array_index) (LocalVariables|GetSpline%20Points)
    (if (== _array_index 0)
      (Utilities|Array|Add (LocalVariables|GetTemp%20Spline%20Points) _array_element)
      (else
        (Utilities|Array|Add _temp_spline_points (Spline|GetLocationatDistanceAlongSpline (Variables|Default|GetSpline) (/ (+ (Spline|GetDistanceAlongSplineatSplinePoint _spline (- _array_index 1)) (Spline|GetDistanceAlongSplineatSplinePoint _spline _array_index)) 2.0) "World"))
        (Utilities|Array|Add _temp_spline_points (Utilities|Array|Get(acopy) (LocalVariables|GetSpline%20Points) _array_index)))))
  (Utilities|Array|Clear (LocalVariables|GetSpline%20Points))
  (return (LocalVariables|GetTemp%20Spline%20Points)))

(fn UnsubdividePoints
  (Utilities|Array|Clear (LocalVariables|GetTemp%20Spline%20Points))
  (for _index (range 0 (- (Spline|GetNumberOfSplinePoints (Variables|Default|GetSpline)) 1))
    (Utilities|Array|Add (LocalVariables|GetSpline%20Points) (Spline|GetLocationatSplinePoint (Variables|Default|GetSpline) _index "World")))
  (if (< (Spline|GetNumberOfSplinePoints (Variables|Default|GetSpline)) 3)
    (return (LocalVariables|GetSpline%20Points))
    (else
      (for (_array_element _array_index) (LocalVariables|GetSpline%20Points)
        (if (== (Math|Integer|%(Integer) _array_index 2) 0)
          (Utilities|Array|Add (LocalVariables|GetTemp%20Spline%20Points) _array_element)))
      (Utilities|Array|Clear (LocalVariables|GetSpline%20Points))
      (return (LocalVariables|GetTemp%20Spline%20Points)))))

(fn BaketoStaticMesh
  (params (FromDynamicMesh :type Dynamic%20Mesh%20Object%20Reference))
  ;[1 1 1] Bake to static mesh
  (if (Variables|Actions|GetBakeToStaticMesh)
    (Variables|Actions|SetBakeToStaticMesh false)
    (bind _returnvalue (Game|GetCurrentLevelName true))
    (bind _output_get (LocalVariables|SetStatic%20Mesh%20Asset%20Path (Utilities|String|Append "/Game/RoadStaticMeshes/" _returnvalue "/" (Utilities|GetDisplayName self))))
    (bind _returnvalue_2 (EditorScripting|Asset|DoesAssetExist _output_get :!class /Script/EditorScriptingUtilities.EditorAssetLibrary))
    (if (not _returnvalue_2)
      (bind _returnvalue_3 (GeometryScript|AssetManagement|CreateNewStaticMeshAssetfromMesh :FromDynamicMesh FromDynamicMesh :AssetPathAndName _output_get :Debug 0) ; Create new asset since it does not exist
        (:Failure
          _)
        (:Success
          (Variables|Default|SetTo%20Static%20Mesh%20Asset _returnvalue_3)
          (Development|PrintString "Success" false :!label _label)
          (return)))
      (else
        (GeometryScript|StaticMesh|CopyMeshtoStaticMesh :FromDynamicMesh FromDynamicMesh :ToStaticMeshAsset (Variables|Default|GetTo%20Static%20Mesh%20Asset) :Debug 0 ; Use existing asset and update it
          (:Failure
            _)
          (:Success
            (goto _label)))))
    (Development|PrintString "Failure to convert to static mesh")
    (return)
    (else
      (return))))

(fn SnaptoGround
  (bind _returnvalue (Transformation|GetActorLocation))
  (bind _trace_distance (Variables|LineOptions|GetTrace%20Distance))
  (for _index (range 0 (- (Spline|GetNumberOfSplinePoints (Variables|Default|GetSpline)) 1))
    (bind _outhit (Collision|LineTraceByChannel (Math|Vector|MakeVector (.x (Spline|GetLocationatSplinePoint (Variables|Default|GetSpline) _index "World")) (.y (Spline|GetLocationatSplinePoint (Variables|Default|GetSpline) _index "World")) (+ (.z _returnvalue) _trace_distance)) (Math|Vector|MakeVector (.x (Spline|GetLocationatSplinePoint (Variables|Default|GetSpline) _index "World")) (.y (Spline|GetLocationatSplinePoint (Variables|Default|GetSpline) _index "World")) (- (.z _returnvalue) _trace_distance)) "TraceTypeQuery1" true (Variables|LineOptions|GetActors%20to%20Ignore) "None"))
    (Spline|SetLocationatSplinePoint (Variables|Default|GetSpline) _index (Math|Vector|MakeVector (.x (Spline|GetLocationatSplinePoint (Variables|Default|GetSpline) _index "World")) (.y (Spline|GetLocationatSplinePoint (Variables|Default|GetSpline) _index "World")) (+ (.z (.location _outhit)) (Variables|LineOptions|GetLine%20Up%20Offset))) "World" true))
  (return))