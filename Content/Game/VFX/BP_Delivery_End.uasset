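; BP_Delivery_End is a delivery end-point objective actor that shows an arrow marker while it is the active objective.
; On becoming active, it spawns a BP_Arrow above its location and stores it in ActiveArrow.
; The objective completed and cleared events both destroy that arrow if it is still valid.
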(event EventBeginPlay
  (|CallParentFunction))

(event Collision|EventActorBeginOverlap
  (params (OtherActor :type Actor%20Object%20Reference)))

(event EventTick
  (params (DeltaSeconds :type Float%20%28single-precision%29)))

(event EventOnBecameActiveObjective
  (bind _returnvalue (Game|SpawnActorfromClass "/Game/Game/VFX/BP_Arrow.BP_Arrow_C" (Math|Transform|MakeTransform (+ (Transformation|GetActorLocation) (Math|Vector|MakeVector 0.0 0.0 3e+02))) "AlwaysSpawn" "MultiplyWithRoot" 0 0))
  (Variables|Default|SetActiveArrow _returnvalue))

(event EventOnObjectiveCompleted
  (bind _activearrow (Variables|Default|GetActiveArrow))
  (Utilities|IsValid _activearrow
    (:Is%20Valid
      (Actor|DestroyActor _activearrow))))

(event EventOnCleared
  (bind _activearrow (Variables|Default|GetActiveArrow))
  (Utilities|IsValid _activearrow
    (:Is%20Valid
      (Actor|DestroyActor _activearrow))))

(fn ConstructionScript
  (|CallParentFunction))